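; Game mode for a two-player, turn-based game that starts play with Blue and Red sides.
; On each login it checks the player count, and at exactly two it tells bp_GameState2 that Blue has the turn.
; It then assigns Blue to the first player's bp_PlayerController2 and Red to the second's, printing an error if either cast fails.
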(event EventBeginPlay)

(event EventTick
  (params (DeltaSeconds :type Float%20%28single-precision%29)))

(event EventPostLogin
  (params (NewPlayer :type Player%20Controller%20Object%20Reference))
  (bind _returnvalue (Class|GameModeBase|GetNumPlayers))
  (if (== _returnvalue 2)
    (Utilities|FlowControl|Sequence
      (:then_0
        (bind _asbp_game_state_2 (Utilities|Casting|CastTobp_GameState2 (Game|GetGameState)))
        (Default|CeGameStateSetPlayerTurn _asbp_game_state_2 "Blue"))
      (:then_1
        (bind _asbp_player_controller_2 (Utilities|Casting|CastTobp_PlayerController2 (Utilities|GetPlayer))
          (:then
            (Default|MyCustomSetPlayerColor(Client) _asbp_player_controller_2 "Blue"))
          (:CastFailed
            (Development|PrintString "ERRO CONVERSAO BPPLAYERCONTROLLER"))))
      (:then_2
        (bind _asbp_player_controller_2_2 (Utilities|Casting|CastTobp_PlayerController2 (Utilities|GetPlayer 1))
          (:then
            (Default|MyCustomSetPlayerColor(Client) _asbp_player_controller_2_2 "Red"))
          (:CastFailed
            (Development|PrintString "ERRO CONVERSAO BPPLAYERCONTROLLER")))))))

(fn ConstructionScript)