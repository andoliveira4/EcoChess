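; Player controller for a two-player networked chess variant with piece skills, assigning Blue to authority and Red to remote when creating the HUD.
; Tile and piece clicks resolve to a board position, then drive selection, castling and king-safe moves using GameState's turn, status and path data.
; Actions are forwarded to GameState through SwitchHasAuthority wrappers around Client/Server RPCs.
; Keys 1–5 snap the pawn and control rotation to preset camera views.
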(event Custom|MyCustom_SetPlayerColor%20%28Client%29
  (params (color :type String))
  (Networking|SwitchHasAuthority
    (:Authority
      (bind _output_get (Variables|Default|SetmyColor "Blue"))
      (bind _returnvalue (UserInterface|CreateWidget "/Game/Widget/HUD_InGame.HUD_InGame_C" 0 _output_get))
      (UserInterface|Viewport|AddtoViewport _returnvalue 0))
    (:Remote
      (bind _output_get_2 (Variables|Default|SetmyColor "Red"))
      (bind _returnvalue_2 (UserInterface|CreateWidget "/Game/Widget/HUD_InGame.HUD_InGame_C" 0 _output_get_2))
      (UserInterface|Viewport|AddtoViewport _returnvalue_2 0))))

(event Custom|OnClicked_Event_0
  (params (TouchedActor :type Actor%20Object%20Reference) (ButtonPressed :type Key%20Structure :default "None"))
  (bind _asbp_soldier (Utilities|Casting|CastTobp_Soldier TouchedActor))
  (Variables|Default|SetselectedTileName (CallFunction|FunctionAjustInttoString (Utilities|Array|FindItem (Variables|/Game/BluePrints/bp_GameState2.bp_GameState2_C|GetBoard (Variables|Default|GetgameState)) (Utilities|GetDisplayName _asbp_soldier))))
  (Development|PrintString (Utilities|String|Append "Clicked in (Soldier): " (Utilities|GetDisplayName _asbp_soldier) ";"))
  (if (Utilities|Enum|Equal(Enum) (Variables|/Game/BluePrints/bp_GameState2.bp_GameState2_C|GetcurrentSelection (Variables|Default|GetGameState)) "")
    (bind _return (Default|FunctionGetifAnyPieceExistinPosition (Variables|Default|GetgameState) (Variables|Default|GetselectedTileName)))
    (if (and _return (Utilities|Enum|Equal(Enum) (Variables|/Game/BluePrints/bp_GameState2.bp_GameState2_C|GetactivePlayer (Variables|Default|GetGameState)) (Variables|Default|GetmyColor)))
      (bind _piecename (Default|FunctionGetPieceBoardNamebyPosition (Variables|Default|GetGameState) (Variables|Default|GetselectedTileName) :!label _label))
      (bind _output_get (Variables|Default|SetpieceName _piecename))
      (bind _color (Default|FunctionGetPieceColor (Variables|Default|GetGameState) _output_get))
      (if (Utilities|Enum|Equal(Enum) _color (Variables|Default|GetmyColor))
        (bind _return_2 (Default|FunctionCheckifPieceIsHattching (Variables|Default|GetgameState) (Variables|Default|GetpieceName)))
        (if (not _return_2)
          (bind _return_3 (Default|FunctionCheckifPieceIsInvencible (Variables|Default|GetGameState) (Variables|Default|GetpieceName)))
          (if (not _return_3)
            (bind _return_4 (Default|FunctionCheckifPieceIsStunned (Variables|Default|GetGameState) (Variables|Default|GetpieceName)))
            (if (not _return_4)
              (CallFunction|CePlayerControllerSetCurrentSelection (Default|FunctionAjustIntegertoStringPure (Variables|Default|GetgameState) (Variables|Default|GetselectedTileName)))
              (CallFunction|CePlayerControllerGetAvaiblePath (Variables|Default|GetselectedTileName)))))))
    (elif (== (Math|Conversions|ToInteger(Byte) (Variables|/Game/BluePrints/bp_GameState2.bp_GameState2_C|GetcurrentSelection (Variables|Default|GetGameState))) (Math|Conversions|ToInteger(Byte) (Variables|Default|GetselectedTileName)))
      (bind _piecename_2 (Default|FunctionGetPieceBoardNamebyPosition (Variables|Default|GetgameState) (Variables|/Game/BluePrints/bp_GameState2.bp_GameState2_C|GetcurrentSelection (Variables|Default|GetgameState))))
      (if (Utilities|String|Contains _piecename_2 (Variables|Default|GetmyColor))
        (CallFunction|CePlayerControllerSetCurrentSelection)
        (CallFunction|CePlayerControllerGetAvaiblePath)
        (Variables|Default|SetdebugMessage ""))
      (else
        (bind _piecename_3 (Default|FunctionGetPieceBoardNamebyPosition (Variables|Default|GetGameState) (Variables|Default|GetselectedTileName)))
        (if (Utilities|String|Contains _piecename_3 (Variables|Default|GetmyColor))
          (if (Utilities|String|Contains (Variables|/Game/BluePrints/bp_GameState2.bp_GameState2_C|GetavaiblePiecePath (Variables|Default|GetgameState)) (Variables|Default|GetselectedTileName))
            (Development|PrintString "CASTLINGGGGGGGGGGGGGGGGGGGGGGGG")
            (CallFunction|CePlayerControlerExecuteCastling (Variables|/Game/BluePrints/bp_GameState2.bp_GameState2_C|GetcurrentSelection (Variables|Default|GetGameState)) (Variables|Default|GetselectedTileName))
            (Utilities|FlowControl|Delay 0.2)
            (if (Variables|/Game/BluePrints/bp_GameState2.bp_GameState2_C|GetcastlingUnavailable? (Variables|Default|GetgameState))
              (Variables|Default|SetdebugMessage "THIS MOVE WILL PUT YOUR KING BE IN DANGER"))
            (else
              (Variables|Default|SetdebugMessage "")
              (CallFunction|CePlayerControllerSetCurrentSelection)
              (CallFunction|CePlayerControllerGetAvaiblePath)
              (goto _label)))
          (else
            (bind _piecename_4 (Default|FunctionGetPieceBoardNamebyPosition (Variables|Default|GetgameState) (Variables|/Game/BluePrints/bp_GameState2.bp_GameState2_C|GetcurrentSelection (Variables|Default|GetgameState))))
            (if (and (Utilities|String|Contains _piecename_4 (Variables|Default|GetmyColor)) (Utilities|String|Contains (Variables|/Game/BluePrints/bp_GameState2.bp_GameState2_C|GetavaiblePiecePath (Variables|Default|GetgameState)) (Variables|Default|GetselectedTileName)))
              (bind _piecename_5 (Default|FunctionGetPieceBoardNamebyPosition (Variables|Default|GetGameState) (Variables|/Game/BluePrints/bp_GameState2.bp_GameState2_C|GetcurrentSelection (Variables|Default|GetGameState))))
              (Variables|Default|SetpieceName _piecename_5)
              (bind (_kingissafe_ _message) (Default|FunctionCheckGameOver (Variables|Default|GetGameState) (Variables|Default|GetpieceName) (Variables|/Game/BluePrints/bp_GameState2.bp_GameState2_C|GetcurrentSelection (Variables|Default|GetGameState)) (Variables|Default|GetselectedTileName)))
              (if _kingissafe_
                (Variables|Default|SetdebugMessage "")
                (CallFunction|CePlayerControllerSetPieceNewPosition (Variables|/Game/BluePrints/bp_GameState2.bp_GameState2_C|GetcurrentSelection (Variables|Default|GetGameState)) (Variables|Default|GetselectedTileName) (Variables|Default|GetpieceName))
                (else
                  (Variables|Default|SetdebugMessage _message))))))))))

(event Custom|ce_PlayerController_SetDestinySelection
  (params (destinySelection :type String))
  (Networking|SwitchHasAuthority
    (:Authority
      (CallFunction|CePlayerControllerSetDestinySelection(Client) destinySelection))
    (:Remote
      (CallFunction|CePlayerControllerSetDestinySelection(Server) destinySelection))))

(event Custom|ce_PlayerController_GetAvaiblePath%20%28Client%29
  (params (selection :type String))
  (Default|CeGameStateGetSetAvaiblePiecePath (Variables|Default|GetgameState) selection))

(event Custom|ce_PlayerController_SetDestinySelection%20%28Server%29
  (params (destinySelection :type String))
  (Default|CeGameStateSetDestinySelection (Variables|Default|GetgameState) destinySelection))

(event Custom|ce_PlayerController_setPlayerTurn%20%28Client%29
  (params (playerColor :type String))
  (Default|CeGameStateSetPlayerTurn (Variables|Default|GetgameState) playerColor))

(event Custom|ce_PlayerController_SetPieceNewPosition%20%28Server%29
  (params (OldPosition :type String) (NewPosition :type String) (pieceName :type String))
  (Default|CeGameStateSetPieceNewPosition (Variables|Default|GetGameState) OldPosition NewPosition pieceName))

(event Custom|ce_PlayerController_SetPieceNewPosition
  (params (OldPosition :type String) (NewPosition :type String) (pieceName :type String))
  (Networking|SwitchHasAuthority
    (:Authority
      (CallFunction|CePlayerControllerSetPieceNewPosition(Client) OldPosition NewPosition pieceName))
    (:Remote
      (CallFunction|CePlayerControllerSetPieceNewPosition(Server) OldPosition NewPosition pieceName))))

(event Custom|ce_PlayerController_GetAvaiblePath
  (params (selection :type String))
  (Networking|SwitchHasAuthority
    (:Authority
      (CallFunction|CePlayerControllerGetAvaiblePath(Client) selection))
    (:Remote
      (CallFunction|CePlayerControllerGetAvaiblePath(Server) selection))))

(event Custom|ce_PlayerController_SetPieceNewPosition%20%28Client%29
  (params (OldPosition :type String) (NewPosition :type String) (pieceName :type String))
  (Default|CeGameStateSetPieceNewPosition (Variables|Default|GetGameState) OldPosition NewPosition pieceName))

(event Custom|ce_PlayerController_setPlayerTurn
  (params (PlayerColor :type String))
  (Networking|SwitchHasAuthority
    (:Authority
      (CallFunction|CePlayerControllerSetPlayerTurn(Client) PlayerColor))
    (:Remote
      (CallFunction|CePlayerControllerSetPlayerTurn(Server) PlayerColor))))

(event Custom|OnClicked_Event_1
  (params (TouchedActor :type Actor%20Object%20Reference) (ButtonPressed :type Key%20Structure :default "None"))
  (bind _asbp_tower (Utilities|Casting|CastTobp_Tower TouchedActor))
  (Variables|Default|SetselectedTileName (CallFunction|FunctionAjustInttoString (Utilities|Array|FindItem (Variables|/Game/BluePrints/bp_GameState2.bp_GameState2_C|GetBoard (Variables|Default|GetgameState)) (Utilities|GetDisplayName _asbp_tower))))
  (if (Utilities|Enum|Equal(Enum) (Variables|/Game/BluePrints/bp_GameState2.bp_GameState2_C|GetcurrentSelection (Variables|Default|GetGameState)) "")
    (bind _return (Default|FunctionGetifAnyPieceExistinPosition (Variables|Default|GetgameState) (Variables|Default|GetselectedTileName)))
    (if (and _return (Utilities|Enum|Equal(Enum) (Variables|/Game/BluePrints/bp_GameState2.bp_GameState2_C|GetactivePlayer (Variables|Default|GetGameState)) (Variables|Default|GetmyColor)))
      (bind _piecename (Default|FunctionGetPieceBoardNamebyPosition (Variables|Default|GetGameState) (Variables|Default|GetselectedTileName) :!label _label))
      (bind _output_get (Variables|Default|SetpieceName _piecename))
      (bind _color (Default|FunctionGetPieceColor (Variables|Default|GetGameState) _output_get))
      (if (Utilities|Enum|Equal(Enum) _color (Variables|Default|GetmyColor))
        (bind _return_2 (Default|FunctionCheckifPieceIsHattching (Variables|Default|GetgameState) (Variables|Default|GetpieceName)))
        (if (not _return_2)
          (bind _return_3 (Default|FunctionCheckifPieceIsInvencible (Variables|Default|GetGameState) (Variables|Default|GetpieceName)))
          (if (not _return_3)
            (bind _return_4 (Default|FunctionCheckifPieceIsStunned (Variables|Default|GetGameState) (Variables|Default|GetpieceName)))
            (if (not _return_4)
              (CallFunction|CePlayerControllerSetCurrentSelection (Default|FunctionAjustIntegertoStringPure (Variables|Default|GetgameState) (Variables|Default|GetselectedTileName)))
              (CallFunction|CePlayerControllerGetAvaiblePath (Variables|Default|GetselectedTileName)))))))
    (elif (== (Math|Conversions|ToInteger(Byte) (Variables|/Game/BluePrints/bp_GameState2.bp_GameState2_C|GetcurrentSelection (Variables|Default|GetGameState))) (Math|Conversions|ToInteger(Byte) (Variables|Default|GetselectedTileName)))
      (bind _piecename_2 (Default|FunctionGetPieceBoardNamebyPosition (Variables|Default|GetgameState) (Variables|/Game/BluePrints/bp_GameState2.bp_GameState2_C|GetcurrentSelection (Variables|Default|GetgameState))))
      (if (Utilities|String|Contains _piecename_2 (Variables|Default|GetmyColor))
        (CallFunction|CePlayerControllerSetCurrentSelection)
        (CallFunction|CePlayerControllerGetAvaiblePath)
        (Variables|Default|SetdebugMessage ""))
      (else
        (bind _piecename_3 (Default|FunctionGetPieceBoardNamebyPosition (Variables|Default|GetGameState) (Variables|Default|GetselectedTileName)))
        (if (Utilities|String|Contains _piecename_3 (Variables|Default|GetmyColor))
          (if (Utilities|String|Contains (Variables|/Game/BluePrints/bp_GameState2.bp_GameState2_C|GetavaiblePiecePath (Variables|Default|GetgameState)) (Variables|Default|GetselectedTileName))
            (Development|PrintString "CASTLINGGGGGGGGGGGGGGGGGGGGGGGG")
            (CallFunction|CePlayerControlerExecuteCastling (Variables|/Game/BluePrints/bp_GameState2.bp_GameState2_C|GetcurrentSelection (Variables|Default|GetGameState)) (Variables|Default|GetselectedTileName))
            (Utilities|FlowControl|Delay 0.2)
            (if (Variables|/Game/BluePrints/bp_GameState2.bp_GameState2_C|GetcastlingUnavailable? (Variables|Default|GetgameState))
              (Variables|Default|SetdebugMessage "THIS MOVE WILL PUT YOUR KING BE IN DANGER"))
            (else
              (Variables|Default|SetdebugMessage "")
              (CallFunction|CePlayerControllerSetCurrentSelection)
              (CallFunction|CePlayerControllerGetAvaiblePath)
              (goto _label)))
          (else
            (bind _piecename_4 (Default|FunctionGetPieceBoardNamebyPosition (Variables|Default|GetgameState) (Variables|/Game/BluePrints/bp_GameState2.bp_GameState2_C|GetcurrentSelection (Variables|Default|GetgameState))))
            (if (and (Utilities|String|Contains _piecename_4 (Variables|Default|GetmyColor)) (Utilities|String|Contains (Variables|/Game/BluePrints/bp_GameState2.bp_GameState2_C|GetavaiblePiecePath (Variables|Default|GetgameState)) (Variables|Default|GetselectedTileName)))
              (bind _piecename_5 (Default|FunctionGetPieceBoardNamebyPosition (Variables|Default|GetGameState) (Variables|/Game/BluePrints/bp_GameState2.bp_GameState2_C|GetcurrentSelection (Variables|Default|GetGameState))))
              (Variables|Default|SetpieceName _piecename_5)
              (bind (_kingissafe_ _message) (Default|FunctionCheckGameOver (Variables|Default|GetGameState) (Variables|Default|GetpieceName) (Variables|/Game/BluePrints/bp_GameState2.bp_GameState2_C|GetcurrentSelection (Variables|Default|GetGameState)) (Variables|Default|GetselectedTileName)))
              (if _kingissafe_
                (Variables|Default|SetdebugMessage "")
                (CallFunction|CePlayerControllerSetPieceNewPosition (Variables|/Game/BluePrints/bp_GameState2.bp_GameState2_C|GetcurrentSelection (Variables|Default|GetGameState)) (Variables|Default|GetselectedTileName) (Variables|Default|GetpieceName))
                (else
                  (Variables|Default|SetdebugMessage _message))))))))))

(event Custom|ce_PlayerController_SetCurrentSelection
  (params (selection :type String))
  (Networking|SwitchHasAuthority
    (:Authority
      (CallFunction|CePlayerControllerSetCurrentSelection(Client) selection))
    (:Remote
      (CallFunction|CePlayerControllerSetCurrentSelection(Server) selection))))

(event Custom|ce_PlayerController_setPlayerTurn%20%28Server%29
  (params (playerColor :type String))
  (Default|CeGameStateSetPlayerTurn (Variables|Default|GetgameState) playerColor))

(event Custom|OnClicked_Event_2
  (params (TouchedActor :type Actor%20Object%20Reference) (ButtonPressed :type Key%20Structure :default "None"))
  (Variables|Default|SetselectedTileName (CallFunction|FunctionAjustInttoString (Utilities|Array|FindItem (Variables|/Game/BluePrints/bp_GameState2.bp_GameState2_C|GetBoard (Variables|Default|GetgameState)) (Utilities|GetDisplayName TouchedActor))))
  (if (Utilities|Enum|Equal(Enum) (Variables|/Game/BluePrints/bp_GameState2.bp_GameState2_C|GetcurrentSelection (Variables|Default|GetGameState)) "")
    (bind _return (Default|FunctionGetifAnyPieceExistinPosition (Variables|Default|GetgameState) (Variables|Default|GetselectedTileName)))
    (if (and _return (Utilities|Enum|Equal(Enum) (Variables|/Game/BluePrints/bp_GameState2.bp_GameState2_C|GetactivePlayer (Variables|Default|GetGameState)) (Variables|Default|GetmyColor)))
      (bind _piecename (Default|FunctionGetPieceBoardNamebyPosition (Variables|Default|GetGameState) (Variables|Default|GetselectedTileName) :!label _label))
      (bind _output_get (Variables|Default|SetpieceName _piecename))
      (bind _color (Default|FunctionGetPieceColor (Variables|Default|GetGameState) _output_get))
      (if (Utilities|Enum|Equal(Enum) _color (Variables|Default|GetmyColor))
        (bind _return_2 (Default|FunctionCheckifPieceIsHattching (Variables|Default|GetgameState) (Variables|Default|GetpieceName)))
        (if (not _return_2)
          (bind _return_3 (Default|FunctionCheckifPieceIsInvencible (Variables|Default|GetGameState) (Variables|Default|GetpieceName)))
          (if (not _return_3)
            (bind _return_4 (Default|FunctionCheckifPieceIsStunned (Variables|Default|GetGameState) (Variables|Default|GetpieceName)))
            (if (not _return_4)
              (CallFunction|CePlayerControllerSetCurrentSelection (Default|FunctionAjustIntegertoStringPure (Variables|Default|GetgameState) (Variables|Default|GetselectedTileName)))
              (CallFunction|CePlayerControllerGetAvaiblePath (Variables|Default|GetselectedTileName)))))))
    (elif (== (Math|Conversions|ToInteger(Byte) (Variables|/Game/BluePrints/bp_GameState2.bp_GameState2_C|GetcurrentSelection (Variables|Default|GetGameState))) (Math|Conversions|ToInteger(Byte) (Variables|Default|GetselectedTileName)))
      (bind _piecename_2 (Default|FunctionGetPieceBoardNamebyPosition (Variables|Default|GetgameState) (Variables|/Game/BluePrints/bp_GameState2.bp_GameState2_C|GetcurrentSelection (Variables|Default|GetgameState))))
      (if (Utilities|String|Contains _piecename_2 (Variables|Default|GetmyColor))
        (CallFunction|CePlayerControllerSetCurrentSelection)
        (CallFunction|CePlayerControllerGetAvaiblePath)
        (Variables|Default|SetdebugMessage ""))
      (else
        (bind _piecename_3 (Default|FunctionGetPieceBoardNamebyPosition (Variables|Default|GetGameState) (Variables|Default|GetselectedTileName)))
        (if (Utilities|String|Contains _piecename_3 (Variables|Default|GetmyColor))
          (if (Utilities|String|Contains (Variables|/Game/BluePrints/bp_GameState2.bp_GameState2_C|GetavaiblePiecePath (Variables|Default|GetgameState)) (Variables|Default|GetselectedTileName))
            (Development|PrintString "CASTLINGGGGGGGGGGGGGGGGGGGGGGGG")
            (CallFunction|CePlayerControlerExecuteCastling (Variables|/Game/BluePrints/bp_GameState2.bp_GameState2_C|GetcurrentSelection (Variables|Default|GetGameState)) (Variables|Default|GetselectedTileName))
            (Utilities|FlowControl|Delay 0.2)
            (if (Variables|/Game/BluePrints/bp_GameState2.bp_GameState2_C|GetcastlingUnavailable? (Variables|Default|GetgameState))
              (Variables|Default|SetdebugMessage "THIS MOVE WILL PUT YOUR KING BE IN DANGER"))
            (else
              (Variables|Default|SetdebugMessage "")
              (CallFunction|CePlayerControllerSetCurrentSelection)
              (CallFunction|CePlayerControllerGetAvaiblePath)
              (goto _label)))
          (else
            (bind _piecename_4 (Default|FunctionGetPieceBoardNamebyPosition (Variables|Default|GetgameState) (Variables|/Game/BluePrints/bp_GameState2.bp_GameState2_C|GetcurrentSelection (Variables|Default|GetgameState))))
            (if (and (Utilities|String|Contains _piecename_4 (Variables|Default|GetmyColor)) (Utilities|String|Contains (Variables|/Game/BluePrints/bp_GameState2.bp_GameState2_C|GetavaiblePiecePath (Variables|Default|GetgameState)) (Variables|Default|GetselectedTileName)))
              (bind _piecename_5 (Default|FunctionGetPieceBoardNamebyPosition (Variables|Default|GetGameState) (Variables|/Game/BluePrints/bp_GameState2.bp_GameState2_C|GetcurrentSelection (Variables|Default|GetGameState))))
              (Variables|Default|SetpieceName _piecename_5)
              (bind (_kingissafe_ _message) (Default|FunctionCheckGameOver (Variables|Default|GetGameState) (Variables|Default|GetpieceName) (Variables|/Game/BluePrints/bp_GameState2.bp_GameState2_C|GetcurrentSelection (Variables|Default|GetGameState)) (Variables|Default|GetselectedTileName)))
              (if _kingissafe_
                (Variables|Default|SetdebugMessage "")
                (CallFunction|CePlayerControllerSetPieceNewPosition (Variables|/Game/BluePrints/bp_GameState2.bp_GameState2_C|GetcurrentSelection (Variables|Default|GetGameState)) (Variables|Default|GetselectedTileName) (Variables|Default|GetpieceName))
                (else
                  (Variables|Default|SetdebugMessage _message))))))))))

(event Custom|ce_PlayerController
  (if (!= (Utilities|Array|FindItem (Variables|/Game/BluePrints/bp_GameState2.bp_GameState2_C|GetdefeatedPieces (Variables|Default|GetgameState)) "KingBlue") -1)
    (Development|PrintString "VERMELHO VENCEU")
    (elif (!= (Utilities|Array|FindItem (Variables|/Game/BluePrints/bp_GameState2.bp_GameState2_C|GetdefeatedPieces (Variables|Default|GetgameState)) "KingRed") -1)
      (Development|PrintString "AZUL VENCEU"))))

(event Custom|OnClicked_Event_3
  (params (TouchedActor :type Actor%20Object%20Reference) (ButtonPressed :type Key%20Structure :default "None"))
  (Variables|Default|SetselectedTileName (CallFunction|FunctionAjustInttoString (Utilities|Array|FindItem (Variables|/Game/BluePrints/bp_GameState2.bp_GameState2_C|GetBoard (Variables|Default|GetgameState)) (Utilities|GetDisplayName TouchedActor))))
  (if (Utilities|Enum|Equal(Enum) (Variables|/Game/BluePrints/bp_GameState2.bp_GameState2_C|GetcurrentSelection (Variables|Default|GetGameState)) "")
    (bind _return (Default|FunctionGetifAnyPieceExistinPosition (Variables|Default|GetgameState) (Variables|Default|GetselectedTileName)))
    (if (and _return (Utilities|Enum|Equal(Enum) (Variables|/Game/BluePrints/bp_GameState2.bp_GameState2_C|GetactivePlayer (Variables|Default|GetGameState)) (Variables|Default|GetmyColor)))
      (bind _piecename (Default|FunctionGetPieceBoardNamebyPosition (Variables|Default|GetGameState) (Variables|Default|GetselectedTileName) :!label _label))
      (bind _output_get (Variables|Default|SetpieceName _piecename))
      (bind _color (Default|FunctionGetPieceColor (Variables|Default|GetGameState) _output_get))
      (if (Utilities|Enum|Equal(Enum) _color (Variables|Default|GetmyColor))
        (bind _return_2 (Default|FunctionCheckifPieceIsHattching (Variables|Default|GetgameState) (Variables|Default|GetpieceName)))
        (if (not _return_2)
          (bind _return_3 (Default|FunctionCheckifPieceIsInvencible (Variables|Default|GetGameState) (Variables|Default|GetpieceName)))
          (if (not _return_3)
            (bind _return_4 (Default|FunctionCheckifPieceIsStunned (Variables|Default|GetGameState) (Variables|Default|GetpieceName)))
            (if (not _return_4)
              (CallFunction|CePlayerControllerSetCurrentSelection (Default|FunctionAjustIntegertoStringPure (Variables|Default|GetgameState) (Variables|Default|GetselectedTileName)))
              (CallFunction|CePlayerControllerGetAvaiblePath (Variables|Default|GetselectedTileName)))))))
    (elif (== (Math|Conversions|ToInteger(Byte) (Variables|/Game/BluePrints/bp_GameState2.bp_GameState2_C|GetcurrentSelection (Variables|Default|GetGameState))) (Math|Conversions|ToInteger(Byte) (Variables|Default|GetselectedTileName)))
      (bind _piecename_2 (Default|FunctionGetPieceBoardNamebyPosition (Variables|Default|GetgameState) (Variables|/Game/BluePrints/bp_GameState2.bp_GameState2_C|GetcurrentSelection (Variables|Default|GetgameState))))
      (if (Utilities|String|Contains _piecename_2 (Variables|Default|GetmyColor))
        (CallFunction|CePlayerControllerSetCurrentSelection)
        (CallFunction|CePlayerControllerGetAvaiblePath)
        (Variables|Default|SetdebugMessage ""))
      (else
        (bind _piecename_3 (Default|FunctionGetPieceBoardNamebyPosition (Variables|Default|GetGameState) (Variables|Default|GetselectedTileName)))
        (if (Utilities|String|Contains _piecename_3 (Variables|Default|GetmyColor))
          (if (Utilities|String|Contains (Variables|/Game/BluePrints/bp_GameState2.bp_GameState2_C|GetavaiblePiecePath (Variables|Default|GetgameState)) (Variables|Default|GetselectedTileName))
            (Development|PrintString "CASTLINGGGGGGGGGGGGGGGGGGGGGGGG")
            (CallFunction|CePlayerControlerExecuteCastling (Variables|/Game/BluePrints/bp_GameState2.bp_GameState2_C|GetcurrentSelection (Variables|Default|GetGameState)) (Variables|Default|GetselectedTileName))
            (Utilities|FlowControl|Delay 0.2)
            (if (Variables|/Game/BluePrints/bp_GameState2.bp_GameState2_C|GetcastlingUnavailable? (Variables|Default|GetgameState))
              (Variables|Default|SetdebugMessage "THIS MOVE WILL PUT YOUR KING BE IN DANGER"))
            (else
              (Variables|Default|SetdebugMessage "")
              (CallFunction|CePlayerControllerSetCurrentSelection)
              (CallFunction|CePlayerControllerGetAvaiblePath)
              (goto _label)))
          (else
            (bind _piecename_4 (Default|FunctionGetPieceBoardNamebyPosition (Variables|Default|GetgameState) (Variables|/Game/BluePrints/bp_GameState2.bp_GameState2_C|GetcurrentSelection (Variables|Default|GetgameState))))
            (if (and (Utilities|String|Contains _piecename_4 (Variables|Default|GetmyColor)) (Utilities|String|Contains (Variables|/Game/BluePrints/bp_GameState2.bp_GameState2_C|GetavaiblePiecePath (Variables|Default|GetgameState)) (Variables|Default|GetselectedTileName)))
              (bind _piecename_5 (Default|FunctionGetPieceBoardNamebyPosition (Variables|Default|GetGameState) (Variables|/Game/BluePrints/bp_GameState2.bp_GameState2_C|GetcurrentSelection (Variables|Default|GetGameState))))
              (Variables|Default|SetpieceName _piecename_5)
              (bind (_kingissafe_ _message) (Default|FunctionCheckGameOver (Variables|Default|GetGameState) (Variables|Default|GetpieceName) (Variables|/Game/BluePrints/bp_GameState2.bp_GameState2_C|GetcurrentSelection (Variables|Default|GetGameState)) (Variables|Default|GetselectedTileName)))
              (if _kingissafe_
                (Variables|Default|SetdebugMessage "")
                (CallFunction|CePlayerControllerSetPieceNewPosition (Variables|/Game/BluePrints/bp_GameState2.bp_GameState2_C|GetcurrentSelection (Variables|Default|GetGameState)) (Variables|Default|GetselectedTileName) (Variables|Default|GetpieceName))
                (else
                  (Variables|Default|SetdebugMessage _message))))))))))

(event Custom|OnClicked_Event_4
  (params (TouchedActor :type Actor%20Object%20Reference) (ButtonPressed :type Key%20Structure :default "None"))
  (Variables|Default|SetselectedTileName (CallFunction|FunctionAjustInttoString (Utilities|Array|FindItem (Variables|/Game/BluePrints/bp_GameState2.bp_GameState2_C|GetBoard (Variables|Default|GetgameState)) (Utilities|GetDisplayName TouchedActor))))
  (if (Utilities|Enum|Equal(Enum) (Variables|/Game/BluePrints/bp_GameState2.bp_GameState2_C|GetcurrentSelection (Variables|Default|GetGameState)) "")
    (bind _return (Default|FunctionGetifAnyPieceExistinPosition (Variables|Default|GetgameState) (Variables|Default|GetselectedTileName)))
    (if (and _return (Utilities|Enum|Equal(Enum) (Variables|/Game/BluePrints/bp_GameState2.bp_GameState2_C|GetactivePlayer (Variables|Default|GetGameState)) (Variables|Default|GetmyColor)))
      (bind _piecename (Default|FunctionGetPieceBoardNamebyPosition (Variables|Default|GetGameState) (Variables|Default|GetselectedTileName) :!label _label))
      (bind _output_get (Variables|Default|SetpieceName _piecename))
      (bind _color (Default|FunctionGetPieceColor (Variables|Default|GetGameState) _output_get))
      (if (Utilities|Enum|Equal(Enum) _color (Variables|Default|GetmyColor))
        (bind _return_2 (Default|FunctionCheckifPieceIsHattching (Variables|Default|GetgameState) (Variables|Default|GetpieceName)))
        (if (not _return_2)
          (bind _return_3 (Default|FunctionCheckifPieceIsInvencible (Variables|Default|GetGameState) (Variables|Default|GetpieceName)))
          (if (not _return_3)
            (bind _return_4 (Default|FunctionCheckifPieceIsStunned (Variables|Default|GetGameState) (Variables|Default|GetpieceName)))
            (if (not _return_4)
              (CallFunction|CePlayerControllerSetCurrentSelection (Default|FunctionAjustIntegertoStringPure (Variables|Default|GetgameState) (Variables|Default|GetselectedTileName)))
              (CallFunction|CePlayerControllerGetAvaiblePath (Variables|Default|GetselectedTileName)))))))
    (elif (== (Math|Conversions|ToInteger(Byte) (Variables|/Game/BluePrints/bp_GameState2.bp_GameState2_C|GetcurrentSelection (Variables|Default|GetGameState))) (Math|Conversions|ToInteger(Byte) (Variables|Default|GetselectedTileName)))
      (bind _piecename_2 (Default|FunctionGetPieceBoardNamebyPosition (Variables|Default|GetgameState) (Variables|/Game/BluePrints/bp_GameState2.bp_GameState2_C|GetcurrentSelection (Variables|Default|GetgameState))))
      (if (Utilities|String|Contains _piecename_2 (Variables|Default|GetmyColor))
        (CallFunction|CePlayerControllerSetCurrentSelection)
        (CallFunction|CePlayerControllerGetAvaiblePath)
        (Variables|Default|SetdebugMessage ""))
      (else
        (bind _piecename_3 (Default|FunctionGetPieceBoardNamebyPosition (Variables|Default|GetGameState) (Variables|Default|GetselectedTileName)))
        (if (Utilities|String|Contains _piecename_3 (Variables|Default|GetmyColor))
          (if (Utilities|String|Contains (Variables|/Game/BluePrints/bp_GameState2.bp_GameState2_C|GetavaiblePiecePath (Variables|Default|GetgameState)) (Variables|Default|GetselectedTileName))
            (Development|PrintString "CASTLINGGGGGGGGGGGGGGGGGGGGGGGG")
            (CallFunction|CePlayerControlerExecuteCastling (Variables|/Game/BluePrints/bp_GameState2.bp_GameState2_C|GetcurrentSelection (Variables|Default|GetGameState)) (Variables|Default|GetselectedTileName))
            (Utilities|FlowControl|Delay 0.2)
            (if (Variables|/Game/BluePrints/bp_GameState2.bp_GameState2_C|GetcastlingUnavailable? (Variables|Default|GetgameState))
              (Variables|Default|SetdebugMessage "THIS MOVE WILL PUT YOUR KING BE IN DANGER"))
            (else
              (Variables|Default|SetdebugMessage "")
              (CallFunction|CePlayerControllerSetCurrentSelection)
              (CallFunction|CePlayerControllerGetAvaiblePath)
              (goto _label)))
          (else
            (bind _piecename_4 (Default|FunctionGetPieceBoardNamebyPosition (Variables|Default|GetgameState) (Variables|/Game/BluePrints/bp_GameState2.bp_GameState2_C|GetcurrentSelection (Variables|Default|GetgameState))))
            (if (and (Utilities|String|Contains _piecename_4 (Variables|Default|GetmyColor)) (Utilities|String|Contains (Variables|/Game/BluePrints/bp_GameState2.bp_GameState2_C|GetavaiblePiecePath (Variables|Default|GetgameState)) (Variables|Default|GetselectedTileName)))
              (bind _piecename_5 (Default|FunctionGetPieceBoardNamebyPosition (Variables|Default|GetGameState) (Variables|/Game/BluePrints/bp_GameState2.bp_GameState2_C|GetcurrentSelection (Variables|Default|GetGameState))))
              (Variables|Default|SetpieceName _piecename_5)
              (bind (_kingissafe_ _message) (Default|FunctionCheckGameOver (Variables|Default|GetGameState) (Variables|Default|GetpieceName) (Variables|/Game/BluePrints/bp_GameState2.bp_GameState2_C|GetcurrentSelection (Variables|Default|GetGameState)) (Variables|Default|GetselectedTileName)))
              (if _kingissafe_
                (Variables|Default|SetdebugMessage "")
                (CallFunction|CePlayerControllerSetPieceNewPosition (Variables|/Game/BluePrints/bp_GameState2.bp_GameState2_C|GetcurrentSelection (Variables|Default|GetGameState)) (Variables|Default|GetselectedTileName) (Variables|Default|GetpieceName))
                (else
                  (Variables|Default|SetdebugMessage _message))))))))))

(event Custom|OnClicked_Event_5
  (params (TouchedActor :type Actor%20Object%20Reference) (ButtonPressed :type Key%20Structure :default "None"))
  (Variables|Default|SetselectedTileName (CallFunction|FunctionAjustInttoString (Utilities|Array|FindItem (Variables|/Game/BluePrints/bp_GameState2.bp_GameState2_C|GetBoard (Variables|Default|GetgameState)) (Utilities|GetDisplayName TouchedActor))))
  (if (Utilities|Enum|Equal(Enum) (Variables|/Game/BluePrints/bp_GameState2.bp_GameState2_C|GetcurrentSelection (Variables|Default|GetGameState)) "")
    (bind _return (Default|FunctionGetifAnyPieceExistinPosition (Variables|Default|GetgameState) (Variables|Default|GetselectedTileName)))
    (if (and _return (Utilities|Enum|Equal(Enum) (Variables|/Game/BluePrints/bp_GameState2.bp_GameState2_C|GetactivePlayer (Variables|Default|GetGameState)) (Variables|Default|GetmyColor)))
      (bind _piecename (Default|FunctionGetPieceBoardNamebyPosition (Variables|Default|GetGameState) (Variables|Default|GetselectedTileName) :!label _label))
      (bind _output_get (Variables|Default|SetpieceName _piecename))
      (bind _color (Default|FunctionGetPieceColor (Variables|Default|GetGameState) _output_get))
      (if (Utilities|Enum|Equal(Enum) _color (Variables|Default|GetmyColor))
        (bind _return_2 (Default|FunctionCheckifPieceIsHattching (Variables|Default|GetgameState) (Variables|Default|GetpieceName)))
        (if (not _return_2)
          (bind _return_3 (Default|FunctionCheckifPieceIsInvencible (Variables|Default|GetGameState) (Variables|Default|GetpieceName)))
          (if (not _return_3)
            (bind _return_4 (Default|FunctionCheckifPieceIsStunned (Variables|Default|GetGameState) (Variables|Default|GetpieceName)))
            (if (not _return_4)
              (CallFunction|CePlayerControllerSetCurrentSelection (Default|FunctionAjustIntegertoStringPure (Variables|Default|GetgameState) (Variables|Default|GetselectedTileName)))
              (CallFunction|CePlayerControllerGetAvaiblePath (Variables|Default|GetselectedTileName)))))))
    (elif (== (Math|Conversions|ToInteger(Byte) (Variables|/Game/BluePrints/bp_GameState2.bp_GameState2_C|GetcurrentSelection (Variables|Default|GetGameState))) (Math|Conversions|ToInteger(Byte) (Variables|Default|GetselectedTileName)))
      (bind _piecename_2 (Default|FunctionGetPieceBoardNamebyPosition (Variables|Default|GetgameState) (Variables|/Game/BluePrints/bp_GameState2.bp_GameState2_C|GetcurrentSelection (Variables|Default|GetgameState))))
      (if (Utilities|String|Contains _piecename_2 (Variables|Default|GetmyColor))
        (CallFunction|CePlayerControllerSetCurrentSelection)
        (CallFunction|CePlayerControllerGetAvaiblePath)
        (Variables|Default|SetdebugMessage ""))
      (else
        (bind _piecename_3 (Default|FunctionGetPieceBoardNamebyPosition (Variables|Default|GetGameState) (Variables|Default|GetselectedTileName)))
        (if (Utilities|String|Contains _piecename_3 (Variables|Default|GetmyColor))
          (if (Utilities|String|Contains (Variables|/Game/BluePrints/bp_GameState2.bp_GameState2_C|GetavaiblePiecePath (Variables|Default|GetgameState)) (Variables|Default|GetselectedTileName))
            (Development|PrintString "CASTLINGGGGGGGGGGGGGGGGGGGGGGGG")
            (CallFunction|CePlayerControlerExecuteCastling (Variables|/Game/BluePrints/bp_GameState2.bp_GameState2_C|GetcurrentSelection (Variables|Default|GetGameState)) (Variables|Default|GetselectedTileName))
            (Utilities|FlowControl|Delay 0.2)
            (if (Variables|/Game/BluePrints/bp_GameState2.bp_GameState2_C|GetcastlingUnavailable? (Variables|Default|GetgameState))
              (Variables|Default|SetdebugMessage "THIS MOVE WILL PUT YOUR KING BE IN DANGER"))
            (else
              (Variables|Default|SetdebugMessage "")
              (CallFunction|CePlayerControllerSetCurrentSelection)
              (CallFunction|CePlayerControllerGetAvaiblePath)
              (goto _label)))
          (else
            (bind _piecename_4 (Default|FunctionGetPieceBoardNamebyPosition (Variables|Default|GetgameState) (Variables|/Game/BluePrints/bp_GameState2.bp_GameState2_C|GetcurrentSelection (Variables|Default|GetgameState))))
            (if (and (Utilities|String|Contains _piecename_4 (Variables|Default|GetmyColor)) (Utilities|String|Contains (Variables|/Game/BluePrints/bp_GameState2.bp_GameState2_C|GetavaiblePiecePath (Variables|Default|GetgameState)) (Variables|Default|GetselectedTileName)))
              (bind _piecename_5 (Default|FunctionGetPieceBoardNamebyPosition (Variables|Default|GetGameState) (Variables|/Game/BluePrints/bp_GameState2.bp_GameState2_C|GetcurrentSelection (Variables|Default|GetGameState))))
              (Variables|Default|SetpieceName _piecename_5)
              (bind (_kingissafe_ _message) (Default|FunctionCheckGameOver (Variables|Default|GetGameState) (Variables|Default|GetpieceName) (Variables|/Game/BluePrints/bp_GameState2.bp_GameState2_C|GetcurrentSelection (Variables|Default|GetGameState)) (Variables|Default|GetselectedTileName)))
              (if _kingissafe_
                (Variables|Default|SetdebugMessage "")
                (CallFunction|CePlayerControllerSetPieceNewPosition (Variables|/Game/BluePrints/bp_GameState2.bp_GameState2_C|GetcurrentSelection (Variables|Default|GetGameState)) (Variables|Default|GetselectedTileName) (Variables|Default|GetpieceName))
                (else
                  (Variables|Default|SetdebugMessage _message))))))))))

(event Custom|ce_PlayerController_UseSkill%20%28Client%29
  (params (structIndex :type Integer))
  (Default|CeGameStateUseSkill (Variables|Default|GetgameState) structIndex))

(event Custom|ce_PlayerController_ActivateSkillA%20%28Server%29
  (params (pieceName :type String) (meshName :type String))
  (Default|CeGameStateUseSkillA (Variables|Default|GetgameState) pieceName meshName))

(event Custom|ce_PlayerController_ActivateSkillA%20%28Client%29
  (params (pieceName :type String) (meshName :type String))
  (Default|CeGameStateUseSkillA (Variables|Default|GetgameState) pieceName meshName))

(event Custom|ce_PlayerController_ActivateSkillA
  (params (pieceName :type String) (meshName :type String))
  (Networking|SwitchHasAuthority
    (:Authority
      (CallFunction|CePlayerControllerActivateSkillA(Client) pieceName meshName))
    (:Remote
      (CallFunction|CePlayerControllerActivateSkillA(Server) pieceName meshName))))

(event Custom|OnClicked_Tile
  (params (TouchedActor :type Actor%20Object%20Reference) (ButtonPressed :type Key%20Structure :default "None"))
  (bind _asbp_tile (Utilities|Casting|CastTobp_Tile TouchedActor))
  (if (not (Utilities|String|Contains (Variables|/Game/BluePrints/Pieces/bp_Tile.bp_Tile_C|GetmyObjectName _asbp_tile) "Board"))
    (Variables|Default|SetselectedTileName (Variables|/Game/BluePrints/Pieces/bp_Tile.bp_Tile_C|GetmyObjectName _asbp_tile))
    (Development|PrintString (Utilities|String|Append "CAMPO (" (Utilities|GetDisplayName _asbp_tile) ") PEÇA (" (Utilities|Array|Get(acopy) (Variables|/Game/BluePrints/bp_GameState2.bp_GameState2_C|GetBoard (Variables|Default|GetgameState)) (Math|Conversions|ToInteger(Byte) (Variables|Default|GetselectedTileName))) ")") true true "(R=0.000000,G=0.660000,B=1.000000,A=1.000000)" 1e+01)
    (if (Utilities|Enum|Equal(Enum) (Variables|/Game/BluePrints/bp_GameState2.bp_GameState2_C|GetcurrentSelection (Variables|Default|GetGameState)) "")
      (bind _return (Default|FunctionGetifAnyPieceExistinPosition (Variables|Default|GetgameState) (Variables|Default|GetselectedTileName)))
      (if (and _return (Utilities|Enum|Equal(Enum) (Variables|/Game/BluePrints/bp_GameState2.bp_GameState2_C|GetactivePlayer (Variables|Default|GetGameState)) (Variables|Default|GetmyColor)))
        (bind _piecename (Default|FunctionGetPieceBoardNamebyPosition (Variables|Default|GetGameState) (Variables|Default|GetselectedTileName) :!label _label))
        (bind _output_get (Variables|Default|SetpieceName _piecename))
        (bind _color (Default|FunctionGetPieceColor (Variables|Default|GetGameState) _output_get))
        (if (Utilities|Enum|Equal(Enum) _color (Variables|Default|GetmyColor))
          (bind _return_2 (Default|FunctionCheckifPieceIsHattching (Variables|Default|GetgameState) (Variables|Default|GetpieceName)))
          (if (not _return_2)
            (bind _return_3 (Default|FunctionCheckifPieceIsInvencible (Variables|Default|GetGameState) (Variables|Default|GetpieceName)))
            (if (not _return_3)
              (bind _return_4 (Default|FunctionCheckifPieceIsStunned (Variables|Default|GetGameState) (Variables|Default|GetpieceName)))
              (if (not _return_4)
                (CallFunction|CePlayerControllerSetCurrentSelection (Default|FunctionAjustIntegertoStringPure (Variables|Default|GetgameState) (Variables|Default|GetselectedTileName)))
                (CallFunction|CePlayerControllerGetAvaiblePath (Variables|Default|GetselectedTileName)))))))
      (elif (== (Math|Conversions|ToInteger(Byte) (Variables|/Game/BluePrints/bp_GameState2.bp_GameState2_C|GetcurrentSelection (Variables|Default|GetGameState))) (Math|Conversions|ToInteger(Byte) (Variables|Default|GetselectedTileName)))
        (bind _piecename_2 (Default|FunctionGetPieceBoardNamebyPosition (Variables|Default|GetgameState) (Variables|/Game/BluePrints/bp_GameState2.bp_GameState2_C|GetcurrentSelection (Variables|Default|GetgameState))))
        (if (Utilities|String|Contains _piecename_2 (Variables|Default|GetmyColor))
          (CallFunction|CePlayerControllerSetCurrentSelection)
          (CallFunction|CePlayerControllerGetAvaiblePath)
          (Variables|Default|SetdebugMessage ""))
        (else
          (bind _piecename_3 (Default|FunctionGetPieceBoardNamebyPosition (Variables|Default|GetGameState) (Variables|Default|GetselectedTileName)))
          (if (Utilities|String|Contains _piecename_3 (Variables|Default|GetmyColor))
            (if (Utilities|String|Contains (Variables|/Game/BluePrints/bp_GameState2.bp_GameState2_C|GetavaiblePiecePath (Variables|Default|GetgameState)) (Variables|Default|GetselectedTileName))
              (Development|PrintString "CASTLINGGGGGGGGGGGGGGGGGGGGGGGG")
              (CallFunction|CePlayerControlerExecuteCastling (Variables|/Game/BluePrints/bp_GameState2.bp_GameState2_C|GetcurrentSelection (Variables|Default|GetGameState)) (Variables|Default|GetselectedTileName))
              (Utilities|FlowControl|Delay 0.2)
              (if (Variables|/Game/BluePrints/bp_GameState2.bp_GameState2_C|GetcastlingUnavailable? (Variables|Default|GetgameState))
                (Variables|Default|SetdebugMessage "THIS MOVE WILL PUT YOUR KING BE IN DANGER"))
              (else
                (Variables|Default|SetdebugMessage "")
                (CallFunction|CePlayerControllerSetCurrentSelection)
                (CallFunction|CePlayerControllerGetAvaiblePath)
                (goto _label)))
            (else
              (bind _piecename_4 (Default|FunctionGetPieceBoardNamebyPosition (Variables|Default|GetgameState) (Variables|/Game/BluePrints/bp_GameState2.bp_GameState2_C|GetcurrentSelection (Variables|Default|GetgameState))))
              (if (and (Utilities|String|Contains _piecename_4 (Variables|Default|GetmyColor)) (Utilities|String|Contains (Variables|/Game/BluePrints/bp_GameState2.bp_GameState2_C|GetavaiblePiecePath (Variables|Default|GetgameState)) (Variables|Default|GetselectedTileName)))
                (bind _piecename_5 (Default|FunctionGetPieceBoardNamebyPosition (Variables|Default|GetGameState) (Variables|/Game/BluePrints/bp_GameState2.bp_GameState2_C|GetcurrentSelection (Variables|Default|GetGameState))))
                (Variables|Default|SetpieceName _piecename_5)
                (bind (_kingissafe_ _message) (Default|FunctionCheckGameOver (Variables|Default|GetGameState) (Variables|Default|GetpieceName) (Variables|/Game/BluePrints/bp_GameState2.bp_GameState2_C|GetcurrentSelection (Variables|Default|GetGameState)) (Variables|Default|GetselectedTileName)))
                (if _kingissafe_
                  (Variables|Default|SetdebugMessage "")
                  (CallFunction|CePlayerControllerSetPieceNewPosition (Variables|/Game/BluePrints/bp_GameState2.bp_GameState2_C|GetcurrentSelection (Variables|Default|GetGameState)) (Variables|Default|GetselectedTileName) (Variables|Default|GetpieceName))
                  (else
                    (Variables|Default|SetdebugMessage _message)))))))))))

(event Custom|ce_PlayerController_Construtor%20%28Client%29
  (Default|CeGameStateConstrutor (Variables|Default|GetgameState)))

(event Custom|ce_PlayerController_UseSkill
  (params (structIndex :type Integer))
  (Networking|SwitchHasAuthority
    (:Authority
      (CallFunction|CePlayerControllerUseSkill(Client) structIndex))
    (:Remote
      (CallFunction|CePlayerControllerUseSkill(Server) structIndex))))

(event Custom|ce_PlayerController_Construtor%20%28Server%29
  (Development|PrintString "SERVER" true true "(R=0.000000,G=0.660000,B=1.000000,A=1.000000)" 9e+01)
  (Default|CeGameStateConstrutor (Variables|Default|GetgameState)))

(event Custom|ce_PlayerController_UseSkill%20%28Server%29
  (params (structIndex :type Integer))
  (Default|CeGameStateUseSkill (Variables|Default|GetgameState) structIndex))

(event Custom|ce_PlayerController_Construtor
  (Networking|SwitchHasAuthority
    (:Authority
      (CallFunction|CePlayerControllerConstrutor(Client)))
    (:Remote
      (CallFunction|CePlayerControllerConstrutor(Server)))))

(event Custom|ce_PlayerController_CheckIfKingWillBeSafe%20%28Client%29
  (params (pieceName :type String) (OldPosition :type String) (NewPosition :type String))
  (Default|CeGameStateCheckiftheKingWillbeSafewithThisMove (Variables|Default|GetgameState) pieceName OldPosition NewPosition))

(event Custom|ce_PlayerController_CheckIfKingWillBeSafe
  (params (pieceName :type String) (OldPosition :type String) (NewPosition :type String))
  (Networking|SwitchHasAuthority
    (:Authority
      (CallFunction|CePlayerControllerCheckifKingWillbeSafe(Server) pieceName OldPosition NewPosition))
    (:Remote
      (CallFunction|CePlayerControllerCheckifKingWillbeSafe(Client) pieceName OldPosition NewPosition))))

(event Custom|ce_PlayerControler_ExecuteCastling%20%28Server%29
  (params (KingPosition :type String) (TowerPosition :type String))
  (Default|CeGameStateExecuteCastling (Variables|Default|GetgameState) KingPosition TowerPosition))

(event Custom|ce_PlayerController_CheckIfKingWillBeSafe%20%28Server%29
  (params (pieceName :type String) (OldPosition :type String) (NewPosition :type String))
  (Default|CeGameStateCheckiftheKingWillbeSafewithThisMove (Variables|Default|GetgameState) pieceName OldPosition NewPosition))

(event Custom|ce_PlayerControler_ExecuteCastling
  (params (KingPosition :type String) (TowerPosition :type String))
  (Networking|SwitchHasAuthority
    (:Authority
      (CallFunction|CePlayerControlerExecuteCastling(Client) KingPosition TowerPosition))
    (:Remote
      (CallFunction|CePlayerControlerExecuteCastling(Server) KingPosition TowerPosition))))

(event Custom|ce_PlayerController_SetCurrentSelection%20%28Client%29
  (params (selection :type String))
  (Default|CeGameStateSetCurrentSelection (Variables|Default|GetgameState) selection))

(event Custom|ce_PlayerControler__ExecuteCastling%20%28Client%29
  (params (KingPosition :type String) (TowerPosition :type String))
  (Default|CeGameStateExecuteCastling (Variables|Default|GetgameState) KingPosition TowerPosition))

(event Custom|OnEndCursorOver_Event_0
  (params (TouchedActor :type Actor%20Object%20Reference))
  (bind _asbp_tile (Utilities|Casting|CastTobp_Tile TouchedActor))
  (Variables|Default|SetlocalTileHover _asbp_tile))

(event Custom|ce_PlayerController_SetCurrentSelection%20%28Server%29
  (params (selection :type String))
  (Default|CeGameStateSetCurrentSelection (Variables|Default|GetgameState) selection))

(event Custom|ce_PlayerController_GetAvaiblePath%20%28Server%29
  (params (selection :type String))
  (Default|CeGameStateGetSetAvaiblePiecePath (Variables|Default|GetgameState) selection))

(event Custom|OnBeginCursorOver_Tile
  (params (TouchedActor :type Actor%20Object%20Reference))
  (bind _asbp_tile (Utilities|Casting|CastTobp_Tile TouchedActor))
  (bind _output_get (Variables|Default|SetlocalTileHover _asbp_tile))
  (if (and (!= (Math|Conversions|ToInteger(Byte) (Variables|/Game/BluePrints/bp_GameState2.bp_GameState2_C|GetcurrentSelection (Variables|Default|GetGameState))) 0) (Utilities|Enum|NotEqual(Enum) (Variables|/Game/BluePrints/bp_GameState2.bp_GameState2_C|GetcurrentSelection (Variables|Default|GetGameState)) (Variables|/Game/BluePrints/Pieces/bp_Tile.bp_Tile_C|GetmyObjectName (Variables|Default|GetlocalTileHover))))
    (Development|PrintString (Utilities|String|Append "[HOVER] - SelectedPieceName [" (Default|FunctionGetPieceBoardNamebyPositionPure (Variables|Default|GetGameState) (Variables|/Game/BluePrints/bp_GameState2.bp_GameState2_C|GetcurrentSelection (Variables|Default|GetGameState))) "]; " "SelectedTile [" (Variables|Default|GetselectedTileName) "]; " "HoverTile [" (Utilities|GetDisplayName (Variables|Default|GetlocalTileHover)) "]") true true "(R=0.000000,G=0.660000,B=1.000000,A=1.000000)" 1e+01)
    (if (Class|KismetStringLibrary|IsNumeric (Utilities|GetDisplayName (Variables|Default|GetlocalTileHover)))
      (CallFunction|CePlayerControllerCheckifKingWillbeSafe (Default|FunctionGetPieceBoardNamebyPositionPure (Variables|Default|GetGameState) (Variables|/Game/BluePrints/bp_GameState2.bp_GameState2_C|GetcurrentSelection (Variables|Default|GetGameState))) (Variables|Default|GetselectedTileName) (Utilities|GetDisplayName (Variables|Default|GetlocalTileHover))))))

(event Custom|ce_PlayerController_SetDestinySelection%20%28Client%29
  (params (destinySelection :type String))
  (Default|CeGameStateSetDestinySelection (Variables|Default|GetgameState) destinySelection))

(event EventBeginPlay
  (Utilities|FlowControl|Sequence
    (:then_0
      (Variables|Default|SetbShowMouseCursor true)
      (Variables|Default|SetbEnableClickEvents true)
      (Variables|Default|SetbEnableMouseOverEvents false)
      (bind _asbp_game_state_2 (Utilities|Casting|CastTobp_GameState2 (Game|GetGameState)))
      (Variables|Default|SetgameState _asbp_game_state_2))
    (:then_1
      (bind _outactors (Actor|GetAllActorsOfClass "bp_PlayerController2_C"))
      (Pawn|SetControlRotation (Utilities|Array|Get(acopy) _outactors) (Variables|Default|Getcamera0))
      (bind _asbp_default_pawn (Utilities|Casting|CastTobp_defaultPawn (Game|Player|GetPlayerPawn 0)))
      (Transformation|SetActorLocation _asbp_default_pawn "-950.000000,-70.000000,250.000000" false false))
    (:then_2
      (bind _outactors_2 (Actor|GetAllActorsOfClass "/Game/BluePrints/Pieces/bp_Tile.bp_Tile_C"))
      (EventDispatchers|AssignOnClicked _outactors_2 (delegate Custom|OnClicked_Tile)))
    (:then_3
      (bind _outactors_3 (Actor|GetAllActorsOfClass "/Game/BluePrints/Pieces/bp_Tile.bp_Tile_C"))
      (EventDispatchers|AssignOnBeginCursorOver _outactors_3 (delegate Custom|OnBeginCursorOver_Tile)))
    (:then_4)
    (:then_5
      (bind _outactors_4 (Actor|GetAllActorsOfClass "/Game/BluePrints/Pieces/bp_Soldier.bp_Soldier_C"))
      (EventDispatchers|AssignOnClicked _outactors_4 (delegate Custom|OnClicked_Event_0)))
    (:then_6
      (bind _outactors_5 (Actor|GetAllActorsOfClass "/Game/BluePrints/Pieces/bp_Tower.bp_Tower_C"))
      (EventDispatchers|AssignOnClicked _outactors_5 (delegate Custom|OnClicked_Event_1)))
    (:then_7
      (bind _outactors_6 (Actor|GetAllActorsOfClass "/Game/BluePrints/Pieces/bp_Knight.bp_Knight_C"))
      (EventDispatchers|AssignOnClicked _outactors_6 (delegate Custom|OnClicked_Event_2)))
    (:then_8
      (bind _outactors_7 (Actor|GetAllActorsOfClass "/Game/BluePrints/Pieces/bp_Bishop.bp_Bishop_C"))
      (EventDispatchers|AssignOnClicked _outactors_7 (delegate Custom|OnClicked_Event_3)))
    (:then_9
      (bind _outactors_8 (Actor|GetAllActorsOfClass "/Game/BluePrints/Pieces/bp_King.bp_King_C"))
      (EventDispatchers|AssignOnClicked _outactors_8 (delegate Custom|OnClicked_Event_4)))
    (:then_10
      (bind _outactors_9 (Actor|GetAllActorsOfClass "/Game/BluePrints/Pieces/bp_Queen.bp_Queen_C"))
      (EventDispatchers|AssignOnClicked _outactors_9 (delegate Custom|OnClicked_Event_5)))))

(event EventTick
  (params (DeltaSeconds :type Float%20%28single-precision%29)))

(event Input|KeyboardEvents|1
  (params (Key :type Key%20Structure :default "None"))
  (:Pressed
    (bind _asbp_default_pawn (Utilities|Casting|CastTobp_defaultPawn (Game|Player|GetPlayerPawn 0)))
    (Transformation|SetActorLocation _asbp_default_pawn "-810.000000,-70.000000,352.000671" false false)
    (Pawn|SetControlRotation (Variables|Default|Getcamera0))))

(event Input|KeyboardEvents|2
  (params (Key :type Key%20Structure :default "None"))
  (:Pressed
    (bind _asbp_default_pawn (Utilities|Casting|CastTobp_defaultPawn (Game|Player|GetPlayerPawn 0)))
    (Transformation|SetActorLocation _asbp_default_pawn "-60.000000,670.000000,352.000671" false false)
    (Pawn|SetControlRotation (Variables|Default|Getcamera1))))

(event Input|KeyboardEvents|3
  (params (Key :type Key%20Structure :default "None"))
  (:Pressed
    (bind _asbp_default_pawn (Utilities|Casting|CastTobp_defaultPawn (Game|Player|GetPlayerPawn 0)))
    (Transformation|SetActorLocation _asbp_default_pawn "690.000000,-70.000000,352.000671" false false)
    (Pawn|SetControlRotation (Variables|Default|Getcamera2))))

(event Input|KeyboardEvents|4
  (params (Key :type Key%20Structure :default "None"))
  (:Pressed
    (bind _asbp_default_pawn (Utilities|Casting|CastTobp_defaultPawn (Game|Player|GetPlayerPawn 0)))
    (Transformation|SetActorLocation _asbp_default_pawn "-60.000000,-800.000000,352.000671" false false)
    (Pawn|SetControlRotation (Variables|Default|Getcamera3))))

(event Input|KeyboardEvents|5
  (params (Key :type Key%20Structure :default "None"))
  (:Pressed
    (bind _asbp_default_pawn (Utilities|Casting|CastTobp_defaultPawn (Game|Player|GetPlayerPawn 0)))
    (Transformation|SetActorLocation _asbp_default_pawn "0.000000,-70.000000,800.000000" false false)
    (Pawn|SetControlRotation (Variables|Default|Getcamera4))))

(fn ConstructionScript)

(fn FunctionAjustInttoString
  (params (integer :type Integer))
  (bind _returnvalue (Utilities|String|ToString(Integer) integer))
  (if (== integer 1)
    (return (Utilities|String|Append "0" _returnvalue))
    (else
      (return _returnvalue))))