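; bp_Logo is a logo piece actor with a static mesh.
; On BeginPlay it casts the game state to bp_GameState2 and caches it.
; A disconnected branch would set the mesh material to blue or red equipment based on the game state's ActivePlayer, but it never runs, so the logo's material is not changed here.
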(event EventBeginPlay
  (bind _asbp_game_state_2 (Utilities|Casting|CastTobp_GameState2 (Game|GetGameState)))
  (Variables|Default|SetGameState _asbp_game_state_2))

(event Collision|EventActorBeginOverlap
  (params (OtherActor :type Actor%20Object%20Reference)))

(event EventTick
  (params (DeltaSeconds :type Float%20%28single-precision%29)))

(fn ConstructionScript)