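; King piece actor for a board game, skinned in Blue or Red team materials, with a lion king mesh outside single player when its Animal is Lion.
; BeginPlay derives the piece's name from its mesh's display name and uses it to find its place in GameState's board data.
; Tick polls GameState to destroy defeated pieces, slide the mesh to a changed tile and show remaining status turns through StatusInfo meshes.
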(event EventBeginPlay
  (bind _mymesh (Variables|Default|GetMyMesh))
  (bind _mymesh_2 (Variables|Default|GetMyMesh))
  (Variables|Default|SetmyObjectName (.LeftS (Utilities|String|Split (Utilities|GetDisplayName (Variables|Default|GetMyMesh)) ".")))
  (bind _asbp_game_state_2 (Utilities|Casting|CastTobp_GameState2 (Game|GetGameState)))
  (Variables|Default|SetGameState _asbp_game_state_2)
  (bind _asbp_game_instance (Utilities|Casting|CastTobp_GameInstance (Game|GetGameInstance)))
  (if (Variables|/Game/BluePrints/bp_GameInstance.bp_GameInstance_C|GetsinglePlayer? _asbp_game_instance)
    (if (Utilities|String|Contains (Variables|Default|GetmyObjectName) "Blue")
      (Rendering|Material|SetMaterial _mymesh 0 "/Game/Mesh/Custom/_BlueEquipment._BlueEquipment")
      (else
        (Rendering|Material|SetMaterial _mymesh 0 "/Game/Mesh/Custom/_RedEquipment._RedEquipment")))
    (if (not (== (Utilities|Array|FindItem (Variables|/Game/BluePrints/bp_GameState2.bp_GameState2_C|GetBoard (Variables|Default|GetgameState)) (Variables|Default|GetmyObjectName)) -1)) :!label _label
      (CallFunction|FunctionSetCurrentSelection (Utilities|String|ToString(Integer) (Utilities|Array|FindItem (Variables|/Game/BluePrints/bp_GameState2.bp_GameState2_C|GetBoard (Variables|Default|GetgameState)) (Variables|Default|GetmyObjectName)))))
    (else
      (Utilities|FlowControl|Sequence
        (:then_0
          (goto _label))
        (:then_1
          (bind (_array_element _array_index) (Utilities|Array|ForEachLoopwithBreak (Variables|/Game/BluePrints/bp_GameState2.bp_GameState2_C|GetBoardStruct (Variables|Default|GetgameState)) :!label _label_2)
            (:LoopBody
              (bind _output_get (Variables|Default|SetlocalStructPieceItem _array_element))
              (Variables|Default|SetlocalStructId _array_index)
              (if (Utilities|String|Contains (Variables|Default|GetmyObjectName) (.Name (Utilities|Struct|Breakbp_StructPiece _output_get)))
                (goto _label_2 Break)))
            (:Completed
              (if (Utilities|String|Contains (.Animal (Utilities|Struct|Breakbp_StructPiece (Variables|Default|GetlocalStructPieceItem))) "Lion")
                ;[1 1 1] Insert Donkey Mesh
                (Components|StaticMesh|SetStaticMesh (Variables|Default|GetMyMesh) "/Game/Mesh/Custom/KingLion.KingLion")
                (Rendering|Material|SetMaterialbyName (Variables|Default|GetMyMesh) "KingLionSkin" "/Game/Mesh/Custom/KingLionSkin.KingLionSkin")
                (Rendering|Material|SetMaterialbyName (Variables|Default|GetMyMesh) "KingLionHair" "/Game/Mesh/Custom/KingLionHair.KingLionHair")
                (Components|StaticMesh|SetStaticMesh (Variables|Default|GetStatusInfo) 0)
                (if (Utilities|String|Contains (Variables|Default|GetmyObjectName) "Blue")
                  (Rendering|Material|SetMaterialbyName _mymesh_2 "KingLionEquipment" "/Game/Mesh/Custom/_BlueEquipment._BlueEquipment")
                  (else
                    (Rendering|Material|SetMaterialbyName _mymesh_2 "KingLionEquipment" "/Game/Mesh/Custom/_RedEquipment._RedEquipment")))))))))))

(event Collision|EventActorBeginOverlap
  (params (OtherActor :type Actor%20Object%20Reference)))

(event EventTick
  (params (DeltaSeconds :type Float%20%28single-precision%29))
  (bind _localstructid (Variables|Default|GetlocalStructId))
  (bind _gamestate (Variables|Default|GetgameState))
  (bind _gamestate_2 (Variables|Default|GetgameState))
  (bind _localstructid_2 (Variables|Default|GetlocalStructId))
  (bind _gamestate_3 (Variables|Default|GetgameState))
  (bind _mymesh (Variables|Default|GetMyMesh))
  (bind _currentturn (Variables|/Game/BluePrints/bp_GameState2.bp_GameState2_C|GetcurrentTurn _gamestate))
  (bind _boardstruct (Variables|/Game/BluePrints/bp_GameState2.bp_GameState2_C|GetBoardStruct _gamestate_2))
  (bind _boardstruct_2 (Variables|/Game/BluePrints/bp_GameState2.bp_GameState2_C|GetBoardStruct _gamestate_3))
  (bind _output (Utilities|Array|Get(acopy) _boardstruct_2 _localstructid))
  (bind _output_2 (Utilities|Array|Get(acopy) _boardstruct _localstructid_2))
  (bind _status (Utilities|Struct|Breakbp_StructPiece _output_2))
  (bind _statuswilllastuntilturn (Utilities|Struct|Breakbp_StructPiece _output))
  (bind _returnvalue (- _statuswilllastuntilturn _currentturn))
  (bind _returnvalue_2 (+ _returnvalue 1))
  (Utilities|FlowControl|Sequence
    (:then_0
      (if (Utilities|Array|ContainsItem (Variables|/Game/BluePrints/bp_GameState2.bp_GameState2_C|GetdefeatedPieces (Variables|Default|GetgameState)) (Variables|Default|GetmyObjectName))
        (Components|DestroyComponent (Variables|Default|GetStatusInfo))
        (Actor|DestroyActor)
        (elif (and (Utilities|Enum|NotEqual(Enum) (Variables|Default|GetcurrentPosition) "") (Utilities|Enum|NotEqual(Enum) (Utilities|Array|Get(acopy) (Variables|/Game/BluePrints/bp_GameState2.bp_GameState2_C|GetBoard (Variables|Default|GetgameState)) (Math|Conversions|ToInteger(Byte) (Variables|Default|GetcurrentPosition))) (Variables|Default|GetmyObjectName)))
          (CallFunction|FunctionSetCurrentSelection (Utilities|String|ToString(Integer) (Utilities|Array|FindItem (Variables|/Game/BluePrints/bp_GameState2.bp_GameState2_C|GetBoard (Variables|Default|GetgameState)) (Variables|Default|GetmyObjectName))))
          (bind _objtile (Default|FunctionGetTileActor (Variables|Default|GetgameState) (Variables|Default|GetcurrentPosition)))
          (Components|MoveComponentTo _mymesh (+ "0.000000,0.000000,20.000000" (Transformation|GetActorLocation _objtile)) (Variables|/Script/Engine.SceneComponent|GetRelativeRotation _mymesh) false false 0.2 false))))
    (:then_1
      (if (Math|Boolean|ORBoolean (Utilities|Enum|Equal(Enum) _status "NewEnumerator0") (Utilities|Enum|Equal(Enum) _status "NewEnumerator5") (Utilities|Enum|Equal(Enum) _status "NewEnumerator6"))
        (Components|StaticMesh|SetStaticMesh (Variables|Default|GetStatusInfo) 0)
        (elif (== _returnvalue_2 3)
          (Components|StaticMesh|SetStaticMesh (Variables|Default|GetStatusInfo) "/Game/Mesh/Custom/3.3")
          (elif (== _returnvalue_2 2)
            (Components|StaticMesh|SetStaticMesh (Variables|Default|GetStatusInfo) "/Game/Mesh/Custom/2.2")
            (elif (== _returnvalue_2 1)
              (Components|StaticMesh|SetStaticMesh (Variables|Default|GetStatusInfo) "/Game/Mesh/Custom/1.1")
              (else
                (Components|StaticMesh|SetStaticMesh (Variables|Default|GetStatusInfo) 0)))))))))

(fn ConstructionScript)

(fn FunctionSetCurrentSelection
  (params (currentSelection :type String))
  (if (== (Utilities|String|Len currentSelection) 1)
    (Variables|Default|SetcurrentPosition (Utilities|String|Append "0" currentSelection))
    (else
      (Variables|Default|SetcurrentPosition currentSelection))))