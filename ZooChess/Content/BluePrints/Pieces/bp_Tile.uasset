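; Board tile actor for a chess-like game, also covering the "tableBoard" piece, that colours itself to reflect game state.
; BeginPlay takes the tile's name from its mesh and paints the checkerboard by numeric row range and digit parity.
; Tick polls bp_GameState2, substring-matching path strings to show selection and possible moves, otherwise tinting dark tiles and the table by active player.
; King-danger highlighting takes priority, only on Blue's turn in single-player.
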(event EventBeginPlay
  (Utilities|FlowControl|Sequence
    (:then_0
      (bind _asbp_game_state_2 (Utilities|Casting|CastTobp_GameState2 (Game|GetGameState)))
      (Variables|Default|SetGameState _asbp_game_state_2)
      (Variables|Default|SetmyObjectName (.LeftS (Utilities|String|Split (Utilities|GetDisplayName (Variables|Default|GetStaticMesh)) "."))))
    (:then_1
      (CallFunction|FunctionBoardPaint (Variables|Default|GetmyObjectName)))))

(event EventTick
  (params (DeltaSeconds :type Float%20%28single-precision%29))
  (bind _asbp_game_instance (Utilities|Casting|CastTobp_GameInstance (Game|GetGameInstance)))
  (if (and (Variables|/Game/BluePrints/bp_GameInstance.bp_GameInstance_C|GetsinglePlayer? _asbp_game_instance) (Utilities|Enum|Equal(Enum) (Variables|/Game/BluePrints/bp_GameState2.bp_GameState2_C|GetactivePlayer (Variables|Default|GetGameState)) "Blue"))
    (if (Utilities|String|Contains (Variables|/Game/BluePrints/bp_GameState2.bp_GameState2_C|GetavaiblePiecePathKingDanger (Variables|Default|GetGameState)) (Variables|Default|GetmyObjectName))
      (Rendering|Material|SetMaterial (Variables|Default|GetStaticMesh) 0 "/Game/Material/Danger.Danger")
      (else
        (if (and (Utilities|Enum|Equal(Enum) (Variables|Default|GetmyObjectName) (Variables|/Game/BluePrints/bp_GameState2.bp_GameState2_C|GetcurrentSelection (Variables|Default|GetGameState))) (Utilities|Enum|Equal(Enum) (Variables|Default|GetmyObjectName) (Utilities|GetDisplayName self))) :!label _label
          (Rendering|Material|SetMaterial (Variables|Default|GetStaticMesh) 0 "/Game/Material/Selected.Selected")
          (elif (Utilities|String|Contains (Variables|/Game/BluePrints/bp_GameState2.bp_GameState2_C|GetavaiblePiecePath (Variables|Default|GetGameState)) (Variables|Default|GetmyObjectName))
            (Rendering|Material|SetMaterial (Variables|Default|GetStaticMesh) 0 "/Game/Material/PossiblePath.PossiblePath")
            (elif (Variables|Default|GetisBlack)
              (if (Utilities|Enum|Equal(Enum) (Variables|/Game/BluePrints/bp_GameState2.bp_GameState2_C|GetactivePlayer (Variables|Default|GetGameState)) "Blue")
                (Rendering|Material|SetMaterial (Variables|Default|GetStaticMesh) 0 "/Game/Material/Black_Blue.Black_Blue")
                (elif (Utilities|Enum|Equal(Enum) (Variables|/Game/BluePrints/bp_GameState2.bp_GameState2_C|GetactivePlayer (Variables|Default|GetGameState)) "Red")
                  (Rendering|Material|SetMaterial (Variables|Default|GetStaticMesh) 0 "/Game/Material/Black_Red.Black_Red")))
              (elif (Utilities|Enum|NotEqual(Enum) (Variables|Default|GetmyObjectName) "tableBoard")
                (Rendering|Material|SetMaterial (Variables|Default|GetStaticMesh) 0 "/Game/Material/White.White")
                (elif (Utilities|Enum|Equal(Enum) (Variables|/Game/BluePrints/bp_GameState2.bp_GameState2_C|GetactivePlayer (Variables|Default|GetGameState)) "Blue")
                  (Rendering|Material|SetMaterial (Variables|Default|GetStaticMesh) 0 "/Game/Material/Black_Blue.Black_Blue")
                  (elif (Utilities|Enum|Equal(Enum) (Variables|/Game/BluePrints/bp_GameState2.bp_GameState2_C|GetactivePlayer (Variables|Default|GetGameState)) "Red")
                    (Rendering|Material|SetMaterial (Variables|Default|GetStaticMesh) 0 "/Game/Material/Black_Red.Black_Red")))))))))
    (else
      (goto _label))))

(fn ConstructionScript)

(fn FunctionBoardPaint
  (params (myObjectName :type String))
  (bind _output_get (LocalVariables|SetlocalObjName myObjectName))
  (if (Utilities|Enum|NotEqual(Enum) _output_get "tableBoard")
    (if (Math|Boolean|ORBoolean (and (>= (Math|Conversions|ToInteger(Byte) (LocalVariables|GetlocalObjName)) 1) (<= (Math|Conversions|ToInteger(Byte) (LocalVariables|GetlocalObjName)) 8)) (and (>= (Math|Conversions|ToInteger(Byte) (LocalVariables|GetlocalObjName)) 17) (<= (Math|Conversions|ToInteger(Byte) (LocalVariables|GetlocalObjName)) 24)) (and (>= (Math|Conversions|ToInteger(Byte) (LocalVariables|GetlocalObjName)) 33) (<= (Math|Conversions|ToInteger(Byte) (LocalVariables|GetlocalObjName)) 40)) (and (>= (Math|Conversions|ToInteger(Byte) (LocalVariables|GetlocalObjName)) 49) (<= (Math|Conversions|ToInteger(Byte) (LocalVariables|GetlocalObjName)) 56)))
      (if (== (.Remainder (Math|Float|Division(WholeandRemainder) (Math|Conversions|ToFloat(Integer) (Utilities|String|GetSubstring (LocalVariables|GetlocalObjName) 1)) 2.0)) 0.0)
        (Rendering|Material|SetMaterial (Variables|Default|GetStaticMesh) 0 "/Game/Material/Black_Blue.Black_Blue")
        (Variables|Default|SetisBlack true)
        (else
          (Rendering|Material|SetMaterial (Variables|Default|GetStaticMesh) 0 "/Game/Mesh/Material.Material")
          (Variables|Default|SetisWhite true)))
      (elif (== (.Remainder (Math|Float|Division(WholeandRemainder) (Math|Conversions|ToFloat(Integer) (Utilities|String|GetSubstring (LocalVariables|GetlocalObjName) 1)) 2.0)) 0.0)
        (Rendering|Material|SetMaterial (Variables|Default|GetStaticMesh) 0 "/Game/Material/White.White")
        (Variables|Default|SetisWhite true)
        (else
          (Rendering|Material|SetMaterial (Variables|Default|GetStaticMesh) 0 "/Game/Material/Black_Blue.Black_Blue")
          (Variables|Default|SetisBlack true))))
    (elif (Utilities|Enum|Equal(Enum) (LocalVariables|GetlocalObjName) "tableBoard")
      (Rendering|Material|SetMaterial (Variables|Default|GetStaticMesh) 0 "/Game/Mesh/Custom/_BlueEquipment._BlueEquipment"))))