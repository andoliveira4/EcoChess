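; Soldier piece actor for a chess-style board game, with classic chess and animal-piece variants, teamed Blue or Red by its mesh name.
; BeginPlay finds its entry in bp_GameState2's board data and applies team materials, plus an animal mesh outside classic mode.
; Tick polls that state to show status countdowns, hide or move the piece, destroy it when defeated, swap Turtle and chick meshes, position Eggs by their Chicken and gild evolved pieces.
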(event EventBeginPlay
  (bind _mymesh (Variables|Default|GetMyMesh))
  (bind _output_get (Variables|Default|SetmyObjectName (.LeftS (Utilities|String|Split (Utilities|GetDisplayName (Variables|Default|GetMyMesh)) "."))))
  (if (Utilities|String|Contains _output_get "Blue")
    (Variables|Default|SetmyObjectColor "Blue")
    (bind _asbp_game_state_2 (Utilities|Casting|CastTobp_GameState2 (Game|GetGameState) :!label _label))
    (Variables|Default|SetGameState _asbp_game_state_2)
    (if (Variables|/Game/BluePrints/bp_GameState2.bp_GameState2_C|GetisClassicChess (Variables|Default|GetgameState))
      (if (Utilities|String|Contains (Variables|Default|GetmyObjectName) "Blue")
        (Rendering|Material|SetMaterial _mymesh 0 "/Game/Mesh/Custom/_BlueEquipment._BlueEquipment")
        (else
          (Rendering|Material|SetMaterial _mymesh 0 "/Game/Mesh/Custom/_RedEquipment._RedEquipment")))
      (if (not (== (Utilities|Array|FindItem (Variables|/Game/BluePrints/bp_GameState2.bp_GameState2_C|GetBoard (Variables|Default|GetgameState)) (Variables|Default|GetmyObjectName)) -1))
        (CallFunction|FunctionSetCurrentSelection (Utilities|String|ToString(Integer) (Utilities|Array|FindItem (Variables|/Game/BluePrints/bp_GameState2.bp_GameState2_C|GetBoard (Variables|Default|GetgameState)) (Variables|Default|GetmyObjectName)))))
      (else
        (Utilities|FlowControl|Sequence
          (:then_0
            (if (not (== (Utilities|Array|FindItem (Variables|/Game/BluePrints/bp_GameState2.bp_GameState2_C|GetBoard (Variables|Default|GetgameState)) (Variables|Default|GetmyObjectName)) -1))
              (CallFunction|FunctionSetCurrentSelection (Utilities|String|ToString(Integer) (Utilities|Array|FindItem (Variables|/Game/BluePrints/bp_GameState2.bp_GameState2_C|GetBoard (Variables|Default|GetgameState)) (Variables|Default|GetmyObjectName))))))
          (:then_1
            (bind (_array_element _array_index) (Utilities|Array|ForEachLoopwithBreak (Variables|/Game/BluePrints/bp_GameState2.bp_GameState2_C|GetBoardStruct (Variables|Default|GetgameState)) :!label _label_2)
              (:LoopBody
                (bind _output_get_2 (Variables|Default|SetlocalStructPieceItem _array_element))
                (Variables|Default|SetlocalStructId _array_index)
                (if (Utilities|String|Contains (Variables|Default|GetmyObjectName) (.Name (Utilities|Struct|Breakbp_StructPiece _output_get_2)))
                  (Components|StaticMesh|SetStaticMesh (Variables|Default|GetStatusInfo) 0)
                  (goto _label_2 Break)))
              (:Completed
                (if (Utilities|String|Contains (.Animal (Utilities|Struct|Breakbp_StructPiece (Variables|Default|GetlocalStructPieceItem))) "Fox")
                  ;[1 1 1] Insere a Mesh da Raposa
                  (bind _returnvalue (Components|StaticMesh|SetStaticMesh (Variables|Default|GetMyMesh) "/Game/Mesh/Custom/SoldierFox.SoldierFox"))
                  (if _returnvalue
                    (Rendering|Material|SetMaterialbyName (Variables|Default|GetMyMesh) "MyPalleteColors" "/Game/Mesh/Custom/MyPalleteColors.MyPalleteColors")
                    (if (Utilities|String|Contains (Variables|Default|GetmyObjectName) "Blue")
                      (Rendering|Material|SetMaterialbyName (Variables|Default|GetMyMesh) "Equipment" "/Game/Mesh/Custom/_BlueEquipment._BlueEquipment")
                      (else
                        (Rendering|Material|SetMaterialbyName (Variables|Default|GetMyMesh) "Equipment" "/Game/Mesh/Custom/_RedEquipment._RedEquipment"))))
                  (elif (Utilities|String|Contains (.Animal (Utilities|Struct|Breakbp_StructPiece (Variables|Default|GetlocalStructPieceItem))) "Rabbit")
                    ;[1 1 1] Insere a Mesh do Coelho
                    (bind _returnvalue_2 (Components|StaticMesh|SetStaticMesh (Variables|Default|GetMyMesh) "/Game/Mesh/Custom/SoldierRabbit.SoldierRabbit"))
                    (if _returnvalue_2
                      (Rendering|Material|SetMaterialbyName (Variables|Default|GetMyMesh) "MyPalleteColors" "/Game/Mesh/Custom/MyPalleteColors.MyPalleteColors")
                      (if (Utilities|String|Contains (Variables|Default|GetmyObjectName) "Blue")
                        (Rendering|Material|SetMaterialbyName (Variables|Default|GetMyMesh) "Equipment" "/Game/Mesh/Custom/_BlueEquipment._BlueEquipment")
                        (else
                          (Rendering|Material|SetMaterialbyName (Variables|Default|GetMyMesh) "Equipment" "/Game/Mesh/Custom/_RedEquipment._RedEquipment"))))
                    (elif (Utilities|String|Contains (.Animal (Utilities|Struct|Breakbp_StructPiece (Variables|Default|GetlocalStructPieceItem))) "Turtle")
                      ;[1 1 1] Insere a Mesh da Tartaruga
                      (Components|StaticMesh|SetStaticMesh (Variables|Default|GetMyMesh) "/Game/Mesh/Custom/SoldierTurtle.SoldierTurtle")
                      (Rendering|Material|SetMaterialbyName (Variables|Default|GetMyMesh) "MyPalleteColors" "/Game/Mesh/Custom/MyPalleteColors.MyPalleteColors")
                      (if (Utilities|String|Contains (Variables|Default|GetmyObjectName) "Blue")
                        (Rendering|Material|SetMaterialbyName (Variables|Default|GetMyMesh) "Equipment" "/Game/Mesh/Custom/_BlueEquipment._BlueEquipment")
                        (else
                          (Rendering|Material|SetMaterialbyName (Variables|Default|GetMyMesh) "Equipment" "/Game/Mesh/Custom/_RedEquipment._RedEquipment")))
                      (elif (Utilities|String|Contains (.Animal (Utilities|Struct|Breakbp_StructPiece (Variables|Default|GetlocalStructPieceItem))) "Chicken")
                        ;[1 1 1] Insere a Mesh da Galinha
                        (Components|StaticMesh|SetStaticMesh (Variables|Default|GetMyMesh) "/Game/Mesh/Custom/SoldierChiken.SoldierChiken")
                        (Rendering|Material|SetMaterialbyName (Variables|Default|GetMyMesh) "MyPalleteColors" "/Game/Mesh/Custom/MyPalleteColors.MyPalleteColors")
                        (if (Utilities|String|Contains (Variables|Default|GetmyObjectName) "Blue")
                          (Rendering|Material|SetMaterialbyName (Variables|Default|GetMyMesh) "Equipment" "/Game/Mesh/Custom/_BlueEquipment._BlueEquipment")
                          (else
                            (Rendering|Material|SetMaterialbyName (Variables|Default|GetMyMesh) "Equipment" "/Game/Mesh/Custom/_RedEquipment._RedEquipment")))
                        (elif (Utilities|String|Contains (.Animal (Utilities|Struct|Breakbp_StructPiece (Variables|Default|GetlocalStructPieceItem))) "Frog")
                          ;[1 1 1] Insere a Mesh do Sapo
                          (bind _returnvalue_3 (Components|StaticMesh|SetStaticMesh (Variables|Default|GetMyMesh) "/Game/Mesh/Custom/SoldierFrog.SoldierFrog"))
                          (if _returnvalue_3
                            (Rendering|Material|SetMaterialbyName (Variables|Default|GetMyMesh) "MyPalleteColors" "/Game/Mesh/Custom/MyPalleteColors.MyPalleteColors")
                            (if (Utilities|String|Contains (Variables|Default|GetmyObjectName) "Blue")
                              (Rendering|Material|SetMaterialbyName (Variables|Default|GetMyMesh) "Equipment" "/Game/Mesh/Custom/_BlueEquipment._BlueEquipment")
                              (else
                                (Rendering|Material|SetMaterialbyName (Variables|Default|GetMyMesh) "Equipment" "/Game/Mesh/Custom/_RedEquipment._RedEquipment"))))
                          (elif (Utilities|String|Contains (.Animal (Utilities|Struct|Breakbp_StructPiece (Variables|Default|GetlocalStructPieceItem))) "Crab")
                            ;[1 1 1] Insere a Mesh do carangueijo
                            (bind _returnvalue_4 (Components|StaticMesh|SetStaticMesh (Variables|Default|GetMyMesh) "/Game/Mesh/Custom/SoldierCrab.SoldierCrab"))
                            (if _returnvalue_4
                              (Rendering|Material|SetMaterialbyName (Variables|Default|GetMyMesh) "MyPalleteColors" "/Game/Mesh/Custom/MyPalleteColors.MyPalleteColors")
                              (if (Utilities|String|Contains (Variables|Default|GetmyObjectName) "Blue")
                                (Rendering|Material|SetMaterialbyName (Variables|Default|GetMyMesh) "Equipment" "/Game/Mesh/Custom/_BlueEquipment._BlueEquipment")
                                (else
                                  (Rendering|Material|SetMaterialbyName (Variables|Default|GetMyMesh) "Equipment" "/Game/Mesh/Custom/_RedEquipment._RedEquipment"))))
                            (elif (Utilities|String|Contains (.Animal (Utilities|Struct|Breakbp_StructPiece (Variables|Default|GetlocalStructPieceItem))) "Pig")
                              ;[1 1 1] Insere a mesh do porco
                              (bind _returnvalue_5 (Components|StaticMesh|SetStaticMesh (Variables|Default|GetMyMesh) "/Game/Mesh/Custom/SoldierPig.SoldierPig"))
                              (if _returnvalue_5
                                (Rendering|Material|SetMaterialbyName (Variables|Default|GetMyMesh) "MyPalleteColors" "/Game/Mesh/Custom/MyPalleteColors.MyPalleteColors")
                                (if (Utilities|String|Contains (Variables|Default|GetmyObjectName) "Blue")
                                  (Rendering|Material|SetMaterialbyName (Variables|Default|GetMyMesh) "Equipment" "/Game/Mesh/Custom/_BlueEquipment._BlueEquipment")
                                  (else
                                    (Rendering|Material|SetMaterialbyName (Variables|Default|GetMyMesh) "Equipment" "/Game/Mesh/Custom/_RedEquipment._RedEquipment"))))
                              (elif (Utilities|String|Contains (.Animal (Utilities|Struct|Breakbp_StructPiece (Variables|Default|GetlocalStructPieceItem))) "Wolf")
                                ;[1 1 1] Insere mesh do Lobo
                                (bind _returnvalue_6 (Components|StaticMesh|SetStaticMesh (Variables|Default|GetMyMesh) "/Game/Mesh/Custom/SoldierWolf.SoldierWolf"))
                                (if _returnvalue_6
                                  (Rendering|Material|SetMaterialbyName (Variables|Default|GetMyMesh) "MyPalleteColors" "/Game/Mesh/Custom/MyPalleteColors.MyPalleteColors")
                                  (if (Utilities|String|Contains (Variables|Default|GetmyObjectName) "Blue")
                                    (Rendering|Material|SetMaterialbyName (Variables|Default|GetMyMesh) "Equipment" "/Game/Mesh/Custom/_BlueEquipment._BlueEquipment")
                                    (else
                                      (Rendering|Material|SetMaterialbyName (Variables|Default|GetMyMesh) "Equipment" "/Game/Mesh/Custom/_RedEquipment._RedEquipment"))))
                                (elif (Utilities|String|Contains (.Animal (Utilities|Struct|Breakbp_StructPiece (Variables|Default|GetlocalStructPieceItem))) "Egg")
                                  ;[1 1 1] Insere mesh do Ovo
                                  (bind _returnvalue_7 (Components|StaticMesh|SetStaticMesh (Variables|Default|GetMyMesh) "/Game/Mesh/Custom/SoldierEgg.SoldierEgg"))
                                  (if _returnvalue_7
                                    (Rendering|Material|SetMaterialbyName (Variables|Default|GetMyMesh) "MyPalleteColors" "/Game/Mesh/Custom/MyPalleteColors.MyPalleteColors")
                                    (if (Utilities|String|Contains (Variables|Default|GetmyObjectName) "Blue")
                                      _)))))))))))))))))
    (elif (Utilities|String|Contains (Variables|Default|GetmyObjectName) "Red")
      (Variables|Default|SetmyObjectColor "Red")
      (goto _label)
      (else
        (Development|PrintString (Utilities|String|Append "ESTA PEÇA NÃO POSSUI NENHUMA DAS CORES: " (Utilities|GetDisplayName (Variables|Default|GetMyMesh))))))))

(event Collision|EventActorBeginOverlap
  (params (OtherActor :type Actor%20Object%20Reference)))

(event EventTick
  (params (DeltaSeconds :type Float%20%28single-precision%29))
  (bind _gamestate (Variables|Default|GetgameState))
  (bind _localstructid (Variables|Default|GetlocalStructId))
  (bind _gamestate_2 (Variables|Default|GetgameState))
  (bind _mymesh (Variables|Default|GetMyMesh))
  (bind _localstructid_2 (Variables|Default|GetlocalStructId))
  (bind _localstructid_3 (Variables|Default|GetlocalStructId))
  (bind _gamestate_3 (Variables|Default|GetgameState))
  (bind _mymesh_2 (Variables|Default|GetMyMesh))
  (bind _boardstruct (Variables|/Game/BluePrints/bp_GameState2.bp_GameState2_C|GetBoardStruct _gamestate))
  (bind _boardstruct_2 (Variables|/Game/BluePrints/bp_GameState2.bp_GameState2_C|GetBoardStruct _gamestate_2))
  (bind _boardstruct_3 (Variables|/Game/BluePrints/bp_GameState2.bp_GameState2_C|GetBoardStruct _gamestate_3))
  (bind _output (Utilities|Array|Get(acopy) _boardstruct_2 _localstructid_2))
  (bind _output_2 (Utilities|Array|Get(acopy) _boardstruct_3 _localstructid_3))
  (bind _output_3 (Utilities|Array|Get(acopy) _boardstruct _localstructid))
  (bind (_name _tile _tipo _animal) (Utilities|Struct|Breakbp_StructPiece _output_2))
  (bind (_name_2 _tile_2 _tipo_2 _animal_2 _skillaisavaible_ _skillaispassive_ _skilladescricao _status) (Utilities|Struct|Breakbp_StructPiece _output_3))
  (bind _status_2 (Utilities|Struct|Breakbp_StructPiece _output))
  (Utilities|FlowControl|Sequence
    (:then_0
      (Utilities|FlowControl|Sequence
        (:then_0
          (if (Math|Boolean|ORBoolean (Utilities|Enum|Equal(Enum) _status_2 "NewEnumerator0") (Utilities|Enum|Equal(Enum) _status_2 "NewEnumerator5") (Utilities|Enum|Equal(Enum) _status_2 "NewEnumerator6"))
            (Components|StaticMesh|SetStaticMesh (Variables|Default|GetStatusInfo) 0)
            (elif (== (+ (Math|Integer|Absolute(Integer) (- (Variables|/Game/BluePrints/bp_GameState2.bp_GameState2_C|GetcurrentTurn (Variables|Default|GetgameState)) (.StatusWillLastUntilTurn (Utilities|Struct|Breakbp_StructPiece (Variables|Default|GetlocalStructPieceItem))))) 1) 3)
              (Components|StaticMesh|SetStaticMesh (Variables|Default|GetStatusInfo) "/Game/Mesh/Custom/3.3")
              (elif (== (+ (Math|Integer|Absolute(Integer) (- (Variables|/Game/BluePrints/bp_GameState2.bp_GameState2_C|GetcurrentTurn (Variables|Default|GetgameState)) (.StatusWillLastUntilTurn (Utilities|Struct|Breakbp_StructPiece (Variables|Default|GetlocalStructPieceItem))))) 1) 2)
                (Components|StaticMesh|SetStaticMesh (Variables|Default|GetStatusInfo) "/Game/Mesh/Custom/2.2")
                (elif (== (+ (Math|Integer|Absolute(Integer) (- (Variables|/Game/BluePrints/bp_GameState2.bp_GameState2_C|GetcurrentTurn (Variables|Default|GetgameState)) (.StatusWillLastUntilTurn (Utilities|Struct|Breakbp_StructPiece (Variables|Default|GetlocalStructPieceItem))))) 1) 1)
                  (Components|StaticMesh|SetStaticMesh (Variables|Default|GetStatusInfo) "/Game/Mesh/Custom/1.1"))))))
        (:then_1
          (if (Utilities|Enum|Equal(Enum) (.Status (Utilities|Struct|Breakbp_StructPiece (Utilities|Array|Get(acopy) (Variables|/Game/BluePrints/bp_GameState2.bp_GameState2_C|GetBoardStruct (Variables|Default|GetgameState)) (Variables|Default|GetlocalStructId)))) "NewEnumerator5")
            (Development|SetHiddeninGame (Variables|Default|GetMyMesh) true false)
            (else
              (Development|SetHiddeninGame (Variables|Default|GetMyMesh) false false))))))
    (:then_1
      (if (Utilities|Array|ContainsItem (Variables|/Game/BluePrints/bp_GameState2.bp_GameState2_C|GetdefeatedPieces (Variables|Default|GetgameState)) (Variables|Default|GetmyObjectName))
        (Components|DestroyComponent (Variables|Default|GetStatusInfo))
        (Actor|DestroyActor)
        (elif (and (Utilities|Enum|NotEqual(Enum) (Variables|Default|GetcurrentPosition) "") (Utilities|Enum|NotEqual(Enum) (Utilities|Array|Get(acopy) (Variables|/Game/BluePrints/bp_GameState2.bp_GameState2_C|GetBoard (Variables|Default|GetgameState)) (Math|Conversions|ToInteger(Byte) (Variables|Default|GetcurrentPosition))) (Variables|Default|GetmyObjectName)))
          (CallFunction|FunctionSetCurrentSelection (Utilities|String|ToString(Integer) (Utilities|Array|FindItem (Variables|/Game/BluePrints/bp_GameState2.bp_GameState2_C|GetBoard (Variables|Default|GetgameState)) (Variables|Default|GetmyObjectName))))
          (bind _objtile (Default|FunctionGetTileActor (Variables|Default|GetgameState) (Variables|Default|GetcurrentPosition)))
          (Components|MoveComponentTo _mymesh_2 (+ "0.000000,0.000000,20.000000" (Transformation|GetActorLocation _objtile)) (Variables|/Script/Engine.SceneComponent|GetRelativeRotation _mymesh_2) true false 0.2 false))))
    (:then_2
      (Variables|Default|SetlocalStructPieceItem (Utilities|Array|Get(acopy) (Variables|/Game/BluePrints/bp_GameState2.bp_GameState2_C|GetBoardStruct (Variables|Default|GetgameState)) (Variables|Default|GetlocalStructId)))
      ;[1 1 1] Checa se a tartaruga esta invencível, se estiver, faz a animação dela se esconder dentro do casco
      (if (Math|Boolean|ANDBoolean (Utilities|Enum|Equal(Enum) (.Name (Utilities|Struct|Breakbp_StructPiece (Variables|Default|GetlocalStructPieceItem))) (Variables|Default|GetmyObjectName)) (Utilities|String|Contains (.Animal (Utilities|Struct|Breakbp_StructPiece (Variables|Default|GetlocalStructPieceItem))) "Turtle") (Utilities|IsValid (Variables|Default|GetMyMesh)))
        (if (Utilities|Enum|Equal(Enum) (.Status (Utilities|Struct|Breakbp_StructPiece (Variables|Default|GetlocalStructPieceItem))) "NewEnumerator1")
          (Components|StaticMesh|SetStaticMesh (Variables|Default|GetMyMesh) "/Game/Mesh/Custom/SoldierTurtleHeadless.SoldierTurtleHeadless")
          (Rendering|Material|SetMaterialbyName (Variables|Default|GetMyMesh) "MyPalleteColors" "/Game/Mesh/Custom/MyPalleteColors.MyPalleteColors")
          (elif (== (Variables|/Script/Engine.StaticMeshComponent|GetStaticMesh _mymesh) "/Game/Mesh/Custom/SoldierTurtleHeadless.SoldierTurtleHeadless")
            (Components|StaticMesh|SetStaticMesh _mymesh "/Game/Mesh/Custom/SoldierTurtle.SoldierTurtle")
            (Rendering|Material|SetMaterialbyName (Variables|Default|GetMyMesh) "MyPalleteColors" "/Game/Mesh/Custom/MyPalleteColors.MyPalleteColors")
            (if (Utilities|String|Contains (Variables|Default|GetmyObjectName) "Blue")
              (Rendering|Material|SetMaterialbyName (Variables|Default|GetMyMesh) "SoldierTurtleEquipment" "/Game/Mesh/Custom/_BlueEquipment._BlueEquipment")
              (else
                (Rendering|Material|SetMaterialbyName (Variables|Default|GetMyMesh) "SoldierTurtleEquipment" "/Game/Mesh/Custom/_RedEquipment._RedEquipment")))))
        (elif (Math|Boolean|ANDBoolean (Utilities|Enum|Equal(Enum) _name_2 (Variables|Default|GetmyObjectName)) (Utilities|String|Contains _animal_2 "Egg") (Utilities|Enum|Equal(Enum) _status "NewEnumerator5") (Utilities|IsValid (Variables|Default|GetMyMesh)))
          (bind _array_element (Utilities|Array|ForEachLoopwithBreak (Variables|/Game/BluePrints/bp_GameState2.bp_GameState2_C|GetBoardStruct (Variables|Default|GetgameState)) :!label _label)
            (:LoopBody
              (if (and (Utilities|String|Contains (.Name (Utilities|Struct|Breakbp_StructPiece _array_element)) (Variables|Default|GetmyObjectColor)) (Utilities|Enum|Equal(Enum) (.Animal (Utilities|Struct|Breakbp_StructPiece _array_element)) "Chicken"))
                (Variables|Default|SetreferencePiece (.Name (Utilities|Struct|Breakbp_StructPiece _array_element)))
                (goto _label Break)))
            (:Completed
              (if (Math|Boolean|Equal(Boolean) (.SkillAisAvaible? (Utilities|Struct|Breakbp_StructPiece _array_element)) true)
                (bind _ajustednumber (Default|FunctionAjustIntegertoString (Variables|Default|GetgameState) (Utilities|String|ToString(Integer) (Utilities|Array|FindItem (Variables|/Game/BluePrints/bp_GameState2.bp_GameState2_C|GetBoard (Variables|Default|GetgameState)) (Variables|Default|GetreferencePiece)))))
                (bind _objtile_2 (Default|FunctionGetTileActor (Variables|Default|GetgameState) _ajustednumber))
                (if (Utilities|Enum|Equal(Enum) (Variables|Default|GetmyObjectColor) "Blue")
                  (Transformation|SetActorLocation (+ "0.000000,0.000000,13.000000" (Transformation|GetActorLocation _objtile_2)) false false)
                  (else
                    (Transformation|SetActorLocation (+ "0.000000,0.000000,13.000000" (Transformation|GetActorLocation _objtile_2)) false false))))))
          (elif (Math|Boolean|ANDBoolean (Utilities|Enum|Equal(Enum) _name (Variables|Default|GetmyObjectName)) (Utilities|Enum|Equal(Enum) _animal "Pintinho") (Utilities|IsValid (Variables|Default|GetMyMesh)))
            (bind _returnvalue (Components|StaticMesh|SetStaticMesh (Variables|Default|GetMyMesh) "/Game/Mesh/Custom/SoldierChick.SoldierChick"))
            (if _returnvalue
              (Rendering|Material|SetMaterialbyName (Variables|Default|GetMyMesh) "SoldierChickSkin" 0)
              (Rendering|Material|SetMaterialbyName (Variables|Default|GetMyMesh) "SoldierChickMouth" 0)
              (if (Utilities|String|Contains (Variables|Default|GetmyObjectName) "Blue")
                (Rendering|Material|SetMaterialbyName (Variables|Default|GetMyMesh) "SoldierChickEquipment" "/Game/Mesh/Custom/_BlueEquipment._BlueEquipment")
                (else
                  (Rendering|Material|SetMaterialbyName (Variables|Default|GetMyMesh) "SoldierChickEquipment" "/Game/Mesh/Custom/_RedEquipment._RedEquipment")))
              (CallFunction|FunctionSetCurrentSelection _tile))))))
    (:then_3
      (bind _output_get (Variables|Default|SetlocalStructPieceItem (Utilities|Array|Get(acopy) (Variables|/Game/BluePrints/bp_GameState2.bp_GameState2_C|GetBoardStruct (Variables|Default|GetgameState)) (Variables|Default|GetlocalStructId))))
      (if (!= (Utilities|Array|FindItem (Variables|/Game/BluePrints/bp_GameState2.bp_GameState2_C|GetdefeatedPieces (Variables|Default|GetgameState)) (.DependOn (Utilities|Struct|Breakbp_StructPiece _output_get))) -1)
        (Actor|DestroyActor)))
    (:then_4
      (if (.Evolved (Utilities|Struct|Breakbp_StructPiece (Variables|Default|GetlocalStructPieceItem)))
        (Utilities|IsValid (Variables|Default|GetMyMesh)
          (:Is%20Valid
            (Rendering|Material|SetMaterialbyName (Variables|Default|GetMyMesh) "Equipment" "/Game/Material/Gold.Gold")
            (Rendering|Material|SetMaterialbyName (Variables|Default|GetMyMesh) "MyPalleteColors" "/Game/Material/Gold.Gold")))))))

(fn ConstructionScript)

(fn FunctionSetCurrentSelection
  (params (currentSelection :type String))
  (if (== (Utilities|String|Len currentSelection) 1)
    (Variables|Default|SetcurrentPosition (Utilities|String|Append "0" currentSelection))
    (else
      (Variables|Default|SetcurrentPosition currentSelection))))